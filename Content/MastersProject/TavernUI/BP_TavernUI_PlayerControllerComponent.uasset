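; Player controller component that manages tavern UI windows through a stack, with toggle, display and hide events that add them to or remove them from the viewport.
; InitComponent opens a test window, shows the mouse cursor and sets Game and UI input.
; A temporary left-click debug key traces under the cursor and displays a hit customer's debug window.
; Displaying increments a Z-order counter, which is never passed to the viewport.
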(event Custom|DisplayWindow
  (params (Window :type User%20Widget%20Object%20Reference))
  (bind _windowstack (Variables|Default|GetWindowStack))
  (if (Utilities|Array|ContainsItem _windowstack Window)
    (Math|Integer|IncrementInt (Variables|Default|GetZOrderIndex))
    (else
      (Utilities|Array|Add _windowstack Window)
      (UserInterface|Viewport|AddtoViewport Window 0)
      (Math|Integer|IncrementInt (Variables|Default|GetZOrderIndex)))))

(event Custom|HideWindow
  (params (Window :type User%20Widget%20Object%20Reference))
  (bind _windowstack (Variables|Default|GetWindowStack))
  (if (Utilities|Array|ContainsItem _windowstack Window)
    (Utilities|Array|RemoveItem _windowstack Window)
    (Widget|RemovefromParent Window)))

(event Custom|ToggleWindow
  (params (Window :type User%20Widget%20Object%20Reference%20%28by%20ref%29))
  (if (Utilities|Array|ContainsItem (Variables|Default|GetWindowStack) Window)
    (CallFunction|HideWindow Window)
    (else
      (CallFunction|DisplayWindow Window))))

(event Custom|InitComponent
  (bind _returnvalue (Game|GetPlayerController 0))
  (bind _returnvalue_2 (UserInterface|CreateWidget "/Game/MastersProject/TavernUI/WBP_TestWindow.WBP_TestWindow_C"))
  (Default|InitialiseWindow _returnvalue_2 _returnvalue_2)
  (CallFunction|ToggleWindow _returnvalue_2)
  (Variables|/Script/Engine.PlayerController|SetbShowMouseCursor _returnvalue true)
  (Input|SetInputModeGameandUI _returnvalue 0 "DoNotLock" false false))

(event Input|MouseEvents|DebugKeyLeftMouseButton
  (params (Key :type Key%20Structure :default "None") (ActionValue :type Input%20Action%20Value%20Structure))
  ;[1 0 0.08255] GET RID OF THIS SOON PLS TY AAAAAAAAAAAAAAAAAA
  (:Pressed
    (bind _asbp_customer (Utilities|Casting|CastToBP_Customer (.HitActor (Collision|BreakHitResult (.HitResult (Class|PlayerController|GetHitResultUnderCursorforObjects (Game|GetPlayerController 0) (Utilities|Array|MakeArray "ObjectTypeQuery2" "ObjectTypeQuery3" "ObjectTypeQuery4") true))))))
    (CallFunction|DisplayWindow (Variables|/Game/MastersProject/Core/Characters/Customer/BP_Customer.BP_Customer_C|GetDEBUGWINDOW _asbp_customer))))
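; Player controller component for the tavern UI that manages a stack of open windows, centred roughly on screen.
; InitComponent shows the cursor, sets game-and-UI input and adds the main mapping context.
; IA_Select line-traces under the mouse and displays the window the hit actor returns; ToggleWindow shows or hides windows.
; Bring-to-front only increments a Z-order counter, as the actual Z-order calls are unconnected.
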(event Custom|DisplayWindow
  (params (Window :type User%20Widget%20Object%20Reference))
  (bind _returnvalue (Viewport|GetViewportSize))
  (bind _windowstack (Variables|Default|GetWindowStack))
  ;[1 0.3008 0.2809] Display Window
  (if (Utilities|Array|ContainsItem _windowstack Window)
    (CallFunction|OrderWindowtoFront Window)
    (else
      (Utilities|Array|Add _windowstack Window)
      (UserInterface|Viewport|AddtoViewport Window 0)
      (Math|Integer|IncrementInt (Variables|Default|GetZOrderIndex)
        (:%20%20
          (Class|UserWidget|SetPositioninViewport Window (Math|Vector2D|MakeVector2D (- (/ (.x _returnvalue) 2.0) 5e+02) (- (/ (.y _returnvalue) 2.0) 2e+02)) true))))))

(event Custom|HideWindow
  (params (Window :type User%20Widget%20Object%20Reference))
  (bind _windowstack (Variables|Default|GetWindowStack))
  ;[1 0.3008 0.2809] Hide Window
  (if (Utilities|Array|ContainsItem _windowstack Window)
    (Utilities|Array|RemoveItem _windowstack Window)
    (Widget|RemovefromParent Window)))

(event Custom|ToggleWindow
  (params (Window :type User%20Widget%20Object%20Reference%20%28by%20ref%29))
  ;[1 0.3008 0.2809] Toggle Window
  (if (Utilities|Array|ContainsItem (Variables|Default|GetWindowStack) Window)
    (CallFunction|HideWindow Window)
    (else
      (CallFunction|DisplayWindow Window))))

(event Custom|InitComponent
  (bind _returnvalue (Game|GetPlayerController 0))
  ;[1 0.8306 0.3224] Init
  (Variables|/Script/Engine.PlayerController|SetbShowMouseCursor _returnvalue true)
  (Input|SetInputModeGameandUI _returnvalue 0 "DoNotLock" false false)
  (Input|AddMappingContext (PlayerController|LocalPlayerSubsystems|GetEnhancedInputLocalPlayerSubsystem (Game|GetPlayerController 0)) "/Game/MastersProject/Core/Input/IMC_Main.IMC_Main" 0 "(bIgnoreAllPressedKeysUntilRelease=True,bForceImmediately=False)"))

(event Custom|OrderWindowToFront
  (params (Window :type User%20Widget%20Object%20Reference))
  ;[1 0.3008 0.2809] Order Window to Front
  (bind _result (Math|Integer|IncrementInt (Variables|Default|GetZOrderIndex))))

(event Input|EnhancedActionEvents|EnhancedInputActionIA_Select
  (params (ActionValue :type Boolean) (ElapsedSeconds :type Float%20%28double-precision%29) (TriggeredSeconds :type Float%20%28double-precision%29) (InputAction :type Input%20Action%20Object%20Reference :default "/Game/MastersProject/Core/Input/IA_Select.IA_Select"))
  (bind _returnvalue (Game|GetPlayerController 0))
  (bind (_worldlocation _worlddirection) (Game|Player|ConvertMouseLocationToWorldSpace _returnvalue))
  ;[0.3226 0.9801 1] Selection
  (:Triggered
    (bind (_outhit _returnvalue_2) (Collision|LineTraceByChannel _worldlocation (+ _worldlocation (* _worlddirection 1e+04)) "TraceTypeQuery2" true 0 "None"))
    (if _returnvalue_2
      (bind _window (Class|BPITavernUI|GetWindow(Message) (.HitActor (Collision|BreakHitResult _outhit))))
      (Utilities|IsValid _window
        (:Is%20Valid
          (CallFunction|DisplayWindow _window))))))
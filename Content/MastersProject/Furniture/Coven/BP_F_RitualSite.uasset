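; BP_F_RitualSite is a Coven furniture Blueprint for a ritual site that shows a Niagara effect during interaction.
; On BeginPlay it binds handlers to the begin and end interact events of its SCFurnitureNeedComponent.
; Beginning an interaction activates the Niagara component without a reset, and ending one deactivates it.
; The construction script only calls its parent.
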(event Custom|OnBeginInteract
  (params (Queue :type Map%20of%20Vectors%20to%20Objects))
  (Components|Activation|Activate (Variables|Default|GetNiagara) false))

(event Custom|OnEndInteract
  (params (Queue :type Map%20of%20Vectors%20to%20Objects))
  (Components|Activation|Deactivate (Variables|Default|GetNiagara)))

(event EventBeginPlay
  (bind _sc_furnitureneedcomponent (Variables|Default|GetSC_FurnitureNeedComponent))
  (EventDispatchers|BindEventtoOnEndInteract _sc_furnitureneedcomponent (delegate Custom|OnEndInteract))
  (EventDispatchers|BindEventtoOnBeginInteract _sc_furnitureneedcomponent (delegate Custom|OnBeginInteract)))

(fn ConstructionScript
  (|CallParentFunction))
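; BP_F_WoodenDoor is a wooden door furniture piece that swings automatically when customers come near.
; A sphere trigger tracks overlapping BP_Customer actors in a CustomersInArea list, ignoring other actor classes.
; Each overlap change plays the DoorRotation timeline while any customer remains and reverses it once the list is empty.
; The timeline alpha drives the DoorHinge relative yaw through a quarter turn.
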(event OnComponentBeginOverlap(Sphere)
  (params (OverlappedComponent :type Primitive%20Component%20Object%20Reference) (OtherActor :type Actor%20Object%20Reference) (OtherComp :type Primitive%20Component%20Object%20Reference) (OtherBodyIndex :type Integer) (bFromSweep :type Boolean) (SweepResult :type Hit%20Result%20Structure%20%28by%20ref%29))
  (if (Utilities|ClassIsChildOf (Utilities|GetClass OtherActor) "/Game/MastersProject/Core/Characters/Customer/BP_Customer.BP_Customer_C")
    (Utilities|Array|Add (Variables|Default|GetCustomersInArea) OtherActor))
  (CallFunction|UpdateDoor))

(event OnComponentEndOverlap(Sphere)
  (params (OverlappedComponent :type Primitive%20Component%20Object%20Reference) (OtherActor :type Actor%20Object%20Reference) (OtherComp :type Primitive%20Component%20Object%20Reference) (OtherBodyIndex :type Integer))
  (if (Utilities|ClassIsChildOf (Utilities|GetClass OtherActor) "/Game/MastersProject/Core/Characters/Customer/BP_Customer.BP_Customer_C")
    (Utilities|Array|RemoveItem (Variables|Default|GetCustomersInArea) OtherActor))
  (CallFunction|UpdateDoor))

(event Custom|UpdateDoor
  (if (> (Utilities|Array|Length (Variables|Default|GetCustomersInArea)) 0)
    (bind _alpha (Timeline|DoorRotation Play)
      (:Update
        (Transformation|SetRelativeRotation (Variables|Default|GetDoorHinge) (Math|Rotator|MakeRotator 0.0 0.0 (+ (* _alpha 9e+01) -9e+01)) false false)))
    (else
      (Timeline|DoorRotation Reverse))))

(fn ConstructionScript)
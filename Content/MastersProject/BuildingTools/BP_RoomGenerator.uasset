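; Room generator building tool that procedurally builds a rectangular room from two corner points and a RoomInfo set of name, meshes and materials.
; Its construction script snaps and orders the corners on a 400-unit grid, derives the tile counts and updates a name label.
; Geometry Script then rebuilds dynamic meshes, tiling the floor across X and Y and repeating wall segments along each edge through a temporary tool mesh.
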(fn ConstructionScript
  (CallFunction|RecalculateRoom))

(fn RecalculateRoom
  (bind _roomname (Variables|Default|GetRoomName))
  ;[1 0.8789 0.2904] Snap Room to Grid & Update Title
  (bind _output_get (Variables|Default|SetCorner1 (Math|Vector|MakeVector (Math|Float|SelectFloat (.x (Class|KismetMathLibrary|VectorSnappedtoGrid (Variables|Default|GetCorner1) 4e+02)) (.x (Class|KismetMathLibrary|VectorSnappedtoGrid (Variables|Default|GetCorner2) 4e+02)) (> (.x (Class|KismetMathLibrary|VectorSnappedtoGrid (Variables|Default|GetCorner1) 4e+02)) (.x (Class|KismetMathLibrary|VectorSnappedtoGrid (Variables|Default|GetCorner2) 4e+02)))) (Math|Float|SelectFloat (.y (Class|KismetMathLibrary|VectorSnappedtoGrid (Variables|Default|GetCorner2) 4e+02)) (.y (Class|KismetMathLibrary|VectorSnappedtoGrid (Variables|Default|GetCorner1) 4e+02)) (> (.y (Class|KismetMathLibrary|VectorSnappedtoGrid (Variables|Default|GetCorner1) 4e+02)) (.y (Class|KismetMathLibrary|VectorSnappedtoGrid (Variables|Default|GetCorner2) 4e+02)))) 0.0)))
  (bind _output_get_2 (Variables|Default|SetCorner2 (Math|Vector|MakeVector (Math|Float|SelectFloat (.x (Class|KismetMathLibrary|VectorSnappedtoGrid (Variables|Default|GetCorner2) 4e+02)) (.x (Class|KismetMathLibrary|VectorSnappedtoGrid (Variables|Default|GetCorner1) 4e+02)) (> (.x (Class|KismetMathLibrary|VectorSnappedtoGrid (Variables|Default|GetCorner1) 4e+02)) (.x (Class|KismetMathLibrary|VectorSnappedtoGrid (Variables|Default|GetCorner2) 4e+02)))) (Math|Float|SelectFloat (.y (Class|KismetMathLibrary|VectorSnappedtoGrid (Variables|Default|GetCorner1) 4e+02)) (.y (Class|KismetMathLibrary|VectorSnappedtoGrid (Variables|Default|GetCorner2) 4e+02)) (> (.y (Class|KismetMathLibrary|VectorSnappedtoGrid (Variables|Default|GetCorner1) 4e+02)) (.y (Class|KismetMathLibrary|VectorSnappedtoGrid (Variables|Default|GetCorner2) 4e+02)))) 0.0)))
  ;[0.2226 1 0.5442] Calculate Room Size
  (Variables|Default|SetRoomSizeX (Math|Integer|Absolute(Integer) (.ReturnValue (Math|Float|Division(WholeandRemainder) (.x (- _output_get _output_get_2)) 4e+02))))
  (Variables|Default|SetRoomSizeY (Math|Integer|Absolute(Integer) (.ReturnValue (Math|Float|Division(WholeandRemainder) (.y (- _output_get _output_get_2)) 4e+02))))
  ;[0.2809 0.3832 1] Add Room Name
  (Transformation|SetWorldLocation _roomname (+ (Variables|Default|GetCorner1) (Transformation|GetActorLocation) "0.000000,0.000000,20.000000") false false)
  (Rendering|Components|TextRender|SetText _roomname (Variables|/Game/MastersProject/BuildingTools/BP_DataAsset_RoomInfo.BP_DataAsset_RoomInfo_C|GetName (Variables|Default|GetRoomInfo)))
  (CallFunction|GenerateFloor)
  (CallFunction|GenerateWalls))

(fn GenerateFloor
  (bind _gridsize (Variables|Default|GetGridSize))
  (bind _returnvalue (/ _gridsize 2))
  (Utilities|IsValid (Variables|Default|GetFloorDynMesh)
    (:Is%20Valid
      (Components|DestroyComponent (Variables|Default|GetFloorDynMesh)))
    (:Is%20Not%20Valid
      _))
  (bind _returnvalue_2 (AddComponent|AddDynamicMeshComponent false))
  (bind _output_get (Variables|Default|SetFloorDynMesh _returnvalue_2))
  (bind _returnvalue_3 (DynamicMeshComponent|GetDynamicMesh _output_get))
  (bind _returnvalue_4 (GeometryScript|StaticMesh|CopyMeshFromStaticMesh :FromStaticMeshAsset (Variables|/Game/MastersProject/BuildingTools/BP_DataAsset_RoomInfo.BP_DataAsset_RoomInfo_C|GetFloorMesh (Variables|Default|GetRoomInfo)) :ToDynamicMesh _returnvalue_3 :Debug 0)
    (:Success
      (bind _returnvalue_5 (Class|GeometryScriptLibraryMeshTransformFunctions|TranslateMesh _returnvalue_4 (+ (Variables|Default|GetCorner1) (Math|Vector|MakeVector (* _returnvalue -1.0) _returnvalue 0.0)) 0))
      (bind _returnvalue_6 (Class|GeometryScriptLibraryMeshBasicEditFunctions|AppendMeshRepeated _returnvalue_5 _returnvalue_5 (Math|Transform|MakeTransform "-400.000000,0.000000,0.000000" "0, 0, 0" "1.000000,1.000000,1.000000") (- (Variables|Default|GetRoomSizeX) 1) true false "(CombineMode=EnableAllMatching)" 0))
      (Class|GeometryScriptLibraryMeshBasicEditFunctions|AppendMeshRepeated _returnvalue_6 _returnvalue_6 (Math|Transform|MakeTransform "0.000000,400.000000,0.000000" "0, 0, 0" "1.000000,1.000000,1.000000") (- (Variables|Default|GetRoomSizeY) 1) true false "(CombineMode=EnableAllMatching)" 0)
      (Rendering|Material|SetMaterial (Variables|Default|GetFloorDynMesh) 0 (Variables|/Game/MastersProject/BuildingTools/BP_DataAsset_RoomInfo.BP_DataAsset_RoomInfo_C|GetFloorMaterial (Variables|Default|GetRoomInfo))))))

(fn GenerateWalls
  (Utilities|IsValid (Variables|Default|GetWallsDynMesh)
    (:Is%20Valid
      (Components|DestroyComponent (Variables|Default|GetWallsDynMesh)))
    (:Is%20Not%20Valid
      _))
  (bind _returnvalue (AddComponent|AddDynamicMeshComponent false))
  (bind _output_get (Variables|Default|SetWallsDynMesh _returnvalue))
  (bind _returnvalue_2 (DynamicMeshComponent|GetDynamicMesh _output_get))
  (LocalVariables|SetWallsDynMeshRef _returnvalue_2)
  (bind _returnvalue_3 (AddComponent|AddDynamicMeshComponent false))
  (bind _output_get_2 (LocalVariables|SetToolDynMesh _returnvalue_3))
  (bind _returnvalue_4 (DynamicMeshComponent|GetDynamicMesh _output_get_2))
  (Utilities|FlowControl|Sequence
    (:then_0
      (CallFunction|AddWallsAlongAxis (LocalVariables|GetWallsDynMeshRef) _returnvalue_4 "0.000000,1.000000,0.000000" (Variables|Default|GetCorner1) (Variables|Default|GetRoomSizeY))
      (CallFunction|AddWallsAlongAxis (LocalVariables|GetWallsDynMeshRef) _returnvalue_4 "-1.000000,0.000000,0.000000" (Variables|Default|GetCorner1) (Variables|Default|GetRoomSizeX))
      (CallFunction|AddWallsAlongAxis (LocalVariables|GetWallsDynMeshRef) _returnvalue_4 "0.000000,-1.000000,0.000000" (Variables|Default|GetCorner2) (Variables|Default|GetRoomSizeY))
      (CallFunction|AddWallsAlongAxis (LocalVariables|GetWallsDynMeshRef) _returnvalue_4 "1.000000,0.000000,0.000000" (Variables|Default|GetCorner2) (Variables|Default|GetRoomSizeX)))
    (:then_1
      (Components|DestroyComponent _returnvalue_3)
      (Rendering|Material|SetMaterial (Variables|Default|GetWallsDynMesh) 0 (Variables|/Game/MastersProject/BuildingTools/BP_DataAsset_RoomInfo.BP_DataAsset_RoomInfo_C|GetWallMaterial (Variables|Default|GetRoomInfo))))))

(fn AddWallsAlongAxis
  (params (WallDynMesh :type Dynamic%20Mesh%20Object%20Reference) (ToolDynMesh :type Dynamic%20Mesh%20Object%20Reference) (Axis :type Vector) (Location :type Vector) (Length :type Integer))
  (bind _gridsize (Variables|Default|GetGridSize))
  (bind _returnvalue (/ _gridsize 2))
  (bind _returnvalue_2 (* _returnvalue 1.0))
  (bind _returnvalue_3 (Math|Vector|MakeVector _returnvalue_2 _returnvalue 0.0))
  (bind _returnvalue_4 (* _returnvalue_3 Axis))
  (bind _returnvalue_5 (+ Location _returnvalue_4))
  (bind _returnvalue_6 (GeometryScript|StaticMesh|CopyMeshFromStaticMesh :FromStaticMeshAsset (Variables|/Game/MastersProject/BuildingTools/BP_DataAsset_RoomInfo.BP_DataAsset_RoomInfo_C|GetWallMesh (Variables|Default|GetRoomInfo)) :ToDynamicMesh ToolDynMesh :Debug 0)
    (:Success
      (bind _returnvalue_7 (Class|GeometryScriptLibraryMeshTransformFunctions|TranslateMesh _returnvalue_6 _returnvalue_5 0))
      (bind _returnvalue_8 (Class|GeometryScriptLibraryMeshTransformFunctions|RotateMesh _returnvalue_7 (Math|Conversions|RotationFromXVector (Math|Vector|VectorGetAbs Axis)) _returnvalue_5 0))
      (Class|GeometryScriptLibraryMeshBasicEditFunctions|AppendMeshRepeated WallDynMesh _returnvalue_8 (Math|Transform|MakeTransform (* Axis (Variables|Default|GetGridSize)) "0, 0, 0" "1.000000,1.000000,1.000000") Length false false "(CombineMode=EnableAllMatching)" 0))))
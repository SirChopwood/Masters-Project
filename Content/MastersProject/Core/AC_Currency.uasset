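; An actor component that holds a currency balance and offers functions to check, add, remove and spend it.
; Spending runs the affordability check first, then deducts the cost and returns true, or returns false without changing the balance.
; Adding and removing both fire an OnCurrencyUpdated dispatcher with the new total, while removing on its own does no balance check.
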(event EventBeginPlay)

(event EventTick
  (params (DeltaSeconds :type Float%20%28single-precision%29)))

(fn HasCurrency
  (params (Cost :type Integer))
  (return (<= Cost (Variables|Default|GetCurrency))))

(fn RemoveCurrency
  (params (Cost :type Integer))
  (bind _output_get (Variables|Default|SetCurrency (- (Variables|Default|GetCurrency) Cost)))
  (Default|CallOnCurrencyUpdated _output_get))

(fn AddCurrency
  (params (CurrencyToAdd :type Integer))
  (bind _output_get (Variables|Default|SetCurrency (+ CurrencyToAdd (Variables|Default|GetCurrency))))
  (Default|CallOnCurrencyUpdated _output_get))

(fn SpendCurrency
  (params (Cost :type Integer))
  (if (CallFunction|HasCurrency Cost)
    (CallFunction|RemoveCurrency Cost)
    (return true)
    (else
      (return false))))
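; Tavern game mode that runs the customer loop and objectives.
; BeginPlay spawns the game manager and player pawn, creates objective and currency UI, starts three objectives and fades in.
; A randomly delayed timer spawns customers at random spawn locations, rescheduling until capacity; each departure triggers another spawn and pays currency on success.
; Spawns progress the customer objective; completed objectives award currency and feed the target-level objective, or print game end when none remain.
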(event Custom|OnCustomerLeave
  (params (Customer :type BP%20Customer%20Object%20Reference) (Success? :type Boolean) (MoneyGained :type Float%20%28double-precision%29))
  (Utilities|Array|RemoveItem (Variables|/Game/MastersProject/Core/BP_GameManager.BP_GameManager_C|GetCustomers (Variables|Default|GetGameManager)) Customer)
  (CallFunction|Spawn)
  (if Success?
    (Default|AddCurrency (Variables|Default|GetAC_Currency) (Math|Float|Ceil MoneyGained) "NewEnumerator1")))

(event Custom|Spawn
  ;[1 1 1] Customer Spawn Timer
  (CallFunction|SpawnCustomer)
  (if (Default|IsValidObjective (Variables|Default|GetGameManager) "/Game/MastersProject/Objectives/DA_Objective_Customers.DA_Objective_Customers")
    (Default|CallOnProgressObjective "/Game/MastersProject/Objectives/DA_Objective_Customers.DA_Objective_Customers" 1))
  (if (< (Utilities|Array|Length (Variables|/Game/MastersProject/Core/BP_GameManager.BP_GameManager_C|GetCustomers (Variables|Default|GetGameManager))) (Variables|Default|GetMaximumCapacity))
    (Utilities|Time|SetTimerbyEvent (EventDispatchers|CreateEvent :!event Custom|Spawn) (Math|Conversions|ToFloat(Integer) (Math|Random|RandomIntegerinRange 5 10)))))

(event Custom|GameEnd
  ;[1 1 1] Game End
  (Development|PrintString "Game End"))

(event Custom|ObjectiveComplete
  (params (ObjectiveData :type PDA%20Objective%20Stats%20Object%20Reference))
  (bind _xpreward (Variables|/Game/MastersProject/Core/Objectives/PDA_ObjectiveStats.PDA_ObjectiveStats_C|GetXPReward ObjectiveData))
  ;[1 1 1] Complete Objective
  (Default|AddCurrency (Variables|Default|GetAC_Currency) _xpreward "NewEnumerator1")
  (if (<= (Utilities|Array|Length (Variables|/Game/MastersProject/Core/BP_GameManager.BP_GameManager_C|GetActiveObjectives (Variables|Default|GetGameManager))) 0)
    (CallFunction|GameEnd)
    (elif (Default|IsValidObjective (Variables|Default|GetGameManager) "/Game/MastersProject/Objectives/DA_Objective_TargetLevel.DA_Objective_TargetLevel")
      (Default|CallOnProgressObjective "/Game/MastersProject/Objectives/DA_Objective_TargetLevel.DA_Objective_TargetLevel" _xpreward))))

(event EventBeginPlay
  ;[1 1 1] Spawn Manager
  (bind _returnvalue (Game|SpawnActorfromClass "/Game/MastersProject/Core/BP_GameManager.BP_GameManager_C" (Math|Transform|MakeTransform "0, 0, 0" "0, 0, 0" "1.000000,1.000000,1.000000") "AdjustIfPossibleButAlwaysSpawn" "MultiplyWithRoot" 0 0))
  (bind _output_get (Variables|Default|SetGameManager _returnvalue))
  (Default|InitManager _output_get self)
  ;[1 1 1] Create UI
  (bind _returnvalue_2 (UserInterface|CreateWidget "/Game/MastersProject/Core/Objectives/WBP_ObjectiveUI.WBP_ObjectiveUI_C"))
  (bind _output_get_2 (Variables|Default|SetObjectiveUI _returnvalue_2))
  (Default|InitUI _output_get_2 self)
  (bind _returnvalue_3 (UserInterface|CreateWidget "/Game/MastersProject/TavernUI/WBP_Currency.WBP_Currency_C"))
  (Variables|Default|SetCurrencyUI _returnvalue_3)
  ;[1 1 1] Spawn Player
  (bind _returnvalue_4 (Game|SpawnActorfromClass "/Game/MastersProject/Core/Characters/Player/BP_PlayerPawn.BP_PlayerPawn_C" (Math|Transform|MakeTransform "0, 0, 0" "0, 0, 0" "1.000000,1.000000,1.000000") "AdjustIfPossibleButAlwaysSpawn" "MultiplyWithRoot" 0 0))
  (Pawn|Possess (Game|GetPlayerController 0) _returnvalue_4)
  (UserInterface|Viewport|AddtoViewport (Variables|Default|GetObjectiveUI) 0)
  (EventDispatchers|BindEventtoOnCompleteObjective (EventDispatchers|CreateEvent :!event Custom|ObjectiveComplete))
  (Default|CallOnStartObjective "/Game/MastersProject/Objectives/DA_Objective_Customers.DA_Objective_Customers")
  (bind _outactors (Actor|GetAllActorsOfClass "/Game/MastersProject/Core/Characters/Customer/BP_CustomerSpawnLocation.BP_CustomerSpawnLocation_C"))
  (Variables|Default|SetSpawners _outactors)
  (bind _returnvalue_5 (Utilities|Time|SetTimerbyEvent (EventDispatchers|CreateEvent :!event Custom|Spawn) (Math|Conversions|ToFloat(Integer) (Math|Random|RandomIntegerinRange 5 10))))
  (Variables|Default|SetCustomerHandle _returnvalue_5)
  (Default|CallOnStartObjective "/Game/MastersProject/Objectives/DA_Objective_TargetLevel.DA_Objective_TargetLevel")
  (Default|CallOnStartObjective "/Game/MastersProject/Objectives/DA_Objective_XP.DA_Objective_XP")
  (CameraFades|StartCameraFade (Game|GetPlayerCameraManager 0) 1.0 0.0 3.0 "(R=0.000000,G=0.000000,B=0.000000,A=1.000000)" true true))

(fn ConstructionScript)

(fn SpawnCustomer
  (bind _customerreference (Default|SpawnCustomer (.OutItem (Utilities|Array|Random (Variables|Default|GetSpawners))) self))
  (Utilities|Array|AddUnique (Variables|/Game/MastersProject/Core/BP_GameManager.BP_GameManager_C|GetCustomers (Variables|Default|GetGameManager)) _customerreference)
  (Default|CallOnCustomerSpawned _customerreference)
  (EventDispatchers|BindEventtoOnLeaveGuild _customerreference (EventDispatchers|CreateEvent :!event Custom|OnCustomerLeave))
  (return))
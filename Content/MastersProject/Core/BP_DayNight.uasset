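; BP_DayNight is a day/night cycle actor that rotates a light and drives an in-game clock.
; Each Tick pitches the light by delta time scaled by Speed and passes the same value to Clock.
; Clock accumulates scaled seconds into a timespan offset from 17:00 and writes it to the referenced widget.
; A disconnected graph section would swap day and night sky dome materials based on actor rotation, but never runs.
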(event EventTick
  (params (DeltaSeconds :type Float%20%28single-precision%29))
  (bind _speed (Variables|Default|GetSpeed))
  (bind _returnvalue (* DeltaSeconds _speed))
  (CallFunction|Clock _returnvalue)
  (Transformation|AddLocalRotation (Variables|/Script/Engine.Actor|GetRootComponent (Variables|Default|GetLight)) (Math|Rotator|MakeRotator 0.0 _returnvalue 0.0) false false))

(fn ConstructionScript)

(fn Clock
  (params (DeltaSeconds :type Float%20%28double-precision%29))
  (bind _refwidget (Variables|Default|GetRefWIdget))
  (bind _output_get (Variables|Default|SetTick (+ (* DeltaSeconds 2.4e+02) (Variables|Default|GetTick))))
  (bind _output_get_2 (Variables|Default|SetTIme (Math|Timespan|MakeTimespan 0 17 0 (Math|Float|Truncate _output_get))))
  (Utilities|IsValid _refwidget
    (:Is%20Valid
      (Variables|/Game/MastersProject/TavernUI/WBP_DayNight.WBP_DayNight_C|SetTimeWidget _refwidget _output_get_2))))
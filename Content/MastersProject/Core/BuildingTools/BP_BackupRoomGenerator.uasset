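; Room generator actor that builds a rectangular, named room from two grid-snapped corners and RoomInfo meshes and materials.
; RecalculateRoom clears old walls, sets the name text and bounds box, then generates floor tiles, walls and doors.
; Doorways replace wall meshes found by two-way traces through overlapping furniture that requires cutouts.
; It runs on construction and whenever the player's furniture component reports this room among affected backup rooms.
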(event Custom|OnBeginRegeneration
  (params (AffectedRooms :type Array%20of%20BP%20Room%20Generator%20Object%20References) (AffectedBackupRooms :type Array%20of%20BP%20Backup%20Room%20Generator%20Object%20References))
  (if (Utilities|Array|ContainsItem AffectedBackupRooms self)
    (CallFunction|RecalculateRoom)))

(event EventBeginPlay
  (EventDispatchers|BindEventtoOnRoomsBeginRegeneration (Actor|GetComponentbyClass (Game|GetPlayerController 0) "/Game/MastersProject/Core/FurnitureSystem/BP_FurniturePCComponent.BP_FurniturePCComponent_C") (delegate Custom|OnBeginRegeneration)))

(fn ConstructionScript
  (CallFunction|RecalculateRoom))

(fn RecalculateRoom
  (bind _roomname (Variables|Default|GetRoomName))
  (bind _wallcomponents (Variables|Components|GetWallComponents))
  (Utilities|FlowControl|Sequence
    (:then_0
      (for _array_element _wallcomponents
        (Components|DestroyComponent _array_element))
      (Utilities|Array|Clear _wallcomponents))
    (:then_1
      ;[1 0.8789 0.2904] Snap Room to Grid & Update Title
      (bind _output_get (Variables|Default|SetCorner1 (Math|Vector|MakeVector (Math|Float|SelectFloat (.x (Class|KismetMathLibrary|VectorSnappedtoGrid (Variables|Default|GetCorner1) 4e+02)) (.x (Class|KismetMathLibrary|VectorSnappedtoGrid (Variables|Default|GetCorner2) 4e+02)) (> (.x (Class|KismetMathLibrary|VectorSnappedtoGrid (Variables|Default|GetCorner1) 4e+02)) (.x (Class|KismetMathLibrary|VectorSnappedtoGrid (Variables|Default|GetCorner2) 4e+02)))) (Math|Float|SelectFloat (.y (Class|KismetMathLibrary|VectorSnappedtoGrid (Variables|Default|GetCorner2) 4e+02)) (.y (Class|KismetMathLibrary|VectorSnappedtoGrid (Variables|Default|GetCorner1) 4e+02)) (> (.y (Class|KismetMathLibrary|VectorSnappedtoGrid (Variables|Default|GetCorner1) 4e+02)) (.y (Class|KismetMathLibrary|VectorSnappedtoGrid (Variables|Default|GetCorner2) 4e+02)))) 0.0)))
      (bind _output_get_2 (Variables|Default|SetCorner2 (Math|Vector|MakeVector (Math|Float|SelectFloat (.x (Class|KismetMathLibrary|VectorSnappedtoGrid (Variables|Default|GetCorner2) 4e+02)) (.x (Class|KismetMathLibrary|VectorSnappedtoGrid (Variables|Default|GetCorner1) 4e+02)) (> (.x (Class|KismetMathLibrary|VectorSnappedtoGrid (Variables|Default|GetCorner1) 4e+02)) (.x (Class|KismetMathLibrary|VectorSnappedtoGrid (Variables|Default|GetCorner2) 4e+02)))) (Math|Float|SelectFloat (.y (Class|KismetMathLibrary|VectorSnappedtoGrid (Variables|Default|GetCorner1) 4e+02)) (.y (Class|KismetMathLibrary|VectorSnappedtoGrid (Variables|Default|GetCorner2) 4e+02)) (> (.y (Class|KismetMathLibrary|VectorSnappedtoGrid (Variables|Default|GetCorner1) 4e+02)) (.y (Class|KismetMathLibrary|VectorSnappedtoGrid (Variables|Default|GetCorner2) 4e+02)))) 0.0)))
      ;[0.2226 1 0.5442] Calculate Room Size
      (Variables|Default|SetRoomSizeX (Math|Integer|Absolute(Integer) (.ReturnValue (Math|Float|Division(WholeandRemainder) (.x (- _output_get _output_get_2)) 4e+02))))
      (Variables|Default|SetRoomSizeY (Math|Integer|Absolute(Integer) (.ReturnValue (Math|Float|Division(WholeandRemainder) (.y (- _output_get _output_get_2)) 4e+02)))))
    (:then_2
      ;[0.2809 0.3832 1] Add Room Name
      (Transformation|SetWorldLocation _roomname (+ (Variables|Default|GetCorner1) (Transformation|GetActorLocation) "-65.000000,70.000000,20.000000") false false)
      (Rendering|Components|TextRender|SetText _roomname (Variables|/Game/MastersProject/Core/BuildingTools/PDA_RoomInfo.PDA_RoomInfo_C|GetName (Variables|Default|GetRoomInfo)))
      ;[1 0.4778 0.4579] Add Room Bounds
      (bind _returnvalue (AddComponent|AddBoxComponent false (Math|Transform|MakeTransform (Math|Vector|Lerp(Vector) (Variables|Default|GetCorner1) (Variables|Default|GetCorner2) 0.5) "0, 0, 0" "1.000000,1.000000,1.000000")))
      (bind _output_get_3 (Variables|Default|SetBoundsBox _returnvalue))
      (Collision|SetCollisionResponsetoAllChannels _output_get_3 "ECR_Ignore")
      (Collision|SetCollisionResponsetoChannel _output_get_3 "ECC_GameTraceChannel1" "ECR_Block")
      (Components|Box|SetBoxExtent _output_get_3 (Math|Vector|MakeVector (* (/ (Variables|Default|GetRoomSizeX) 2) 4e+02) (* (/ (Variables|Default|GetRoomSizeY) 2) 4e+02) 5e+02) false)
      (Class|BoxComponent|SetLineThickness _output_get_3 2e+01))
    (:then_3
      (CallFunction|GenerateFloor)
      (CallFunction|GenerateWalls)
      (CallFunction|GenerateDoors))))

(fn GenerateFloor
  (bind _roominfo (Variables|Default|GetRoomInfo))
  (bind _gridsize (Variables|Default|GetGridSize))
  (bind _returnvalue (* _gridsize 0.5))
  (bind _index (Utilities|FlowControl|ForLoopwithBreak 1 (Variables|Default|GetRoomSizeX))
    (:LoopBody
      (bind _index_2 (Utilities|FlowControl|ForLoopwithBreak 1 (Variables|Default|GetRoomSizeY))
        (:LoopBody
          (bind _returnvalue_2 (AddComponent|AddStaticMeshComponent false (Math|Transform|MakeTransform (+ (Variables|Default|GetCorner1) (Math|Vector|MakeVector (* _index _gridsize -1) (* _index_2 _gridsize) 0.0) (Math|Vector|MakeVector _returnvalue (* _returnvalue -1.0) 0.0)) "0, 0, 0" "1.000000,1.000000,1.000000")))
          (Components|StaticMesh|SetStaticMesh _returnvalue_2 (Variables|/Game/MastersProject/Core/BuildingTools/PDA_RoomInfo.PDA_RoomInfo_C|GetFloorMesh _roominfo))
          (Rendering|Material|SetMaterial _returnvalue_2 0 (Variables|/Game/MastersProject/Core/BuildingTools/PDA_RoomInfo.PDA_RoomInfo_C|GetFloorMaterial _roominfo)))))
    (:Completed
      (return))))

(fn GenerateWalls
  (bind _corner2 (Variables|Default|GetCorner2))
  (bind _roomsizey (Variables|Default|GetRoomSizeY))
  (bind _corner1 (Variables|Default|GetCorner1))
  (bind _roomsizex (Variables|Default|GetRoomSizeX))
  ;[1 0.4129 0.2116] Add Wall Sides
  (CallFunction|AddWallsAlongAxis "0.000000,1.000000,0.000000" _corner1 _roomsizey false)
  (CallFunction|AddWallsAlongAxis "-1.000000,0.000000,0.000000" _corner1 _roomsizex false)
  (CallFunction|AddWallsAlongAxis "0.000000,-1.000000,0.000000" _corner2 _roomsizey true)
  (CallFunction|AddWallsAlongAxis "1.000000,0.000000,0.000000" _corner2 _roomsizex true))

(fn AddWallsAlongAxis
  (params (Axis :type Vector) (Location :type Vector) (Length :type Integer) (FlipWall :type Boolean))
  (bind (_x _y) (Class|KismetMathLibrary|BreakVector3f Axis))
  (bind _returnvalue (Math|Vector|VectorGetAbs Axis))
  (bind _gridsize (Variables|Default|GetGridSize))
  (bind _roominfo (Variables|Default|GetRoomInfo))
  (bind _returnvalue_2 (Math|Conversions|RotationFromXVector _returnvalue))
  (bind _returnvalue_3 (/ _gridsize 2))
  (for _index (range 1 Length)
    (bind _returnvalue_4 (AddComponent|AddStaticMeshComponent false (Math|Transform|MakeTransform (+ (+ Location (* (Math|Vector|MakeVector _returnvalue_3 _returnvalue_3 0.0) Axis)) (* (* (Variables|Default|GetGridSize) (- _index 1)) Axis) (* (Math|Vector|MakeVector (* _y -1.0) (* _x -1.0) 0.0) 1e+01)) (Math|Rotator|SelectRotator (Math|Rotator|CombineRotators _returnvalue_2 "0.000000,180.000000,0.000000") _returnvalue_2 FlipWall) "1.000000,1.000000,1.000000")))
    (Components|StaticMesh|SetStaticMesh _returnvalue_4 (Variables|/Game/MastersProject/Core/BuildingTools/PDA_RoomInfo.PDA_RoomInfo_C|GetWallMesh _roominfo))
    (Rendering|Material|SetMaterial _returnvalue_4 0 (Variables|/Game/MastersProject/Core/BuildingTools/PDA_RoomInfo.PDA_RoomInfo_C|GetWallMaterial _roominfo))
    (Collision|SetCollisionProfileName _returnvalue_4 "Walls" true :!class /Script/Engine.PrimitiveComponent)
    (Collision|SetCollisionEnabled _returnvalue_4 "QueryAndPhysics")
    (Utilities|Array|Add (Variables|Components|GetWallComponents) _returnvalue_4)))

(fn GenerateDoors
  (bind _boundsbox (Variables|Default|GetBoundsBox))
  (bind _outactors (Collision|ComponentOverlapActors _boundsbox (Transformation|GetWorldTransform _boundsbox) (Utilities|Array|MakeArray "ObjectTypeQuery7") 0))
  (for _array_element _outactors
    (if (Variables|/Game/MastersProject/Core/FurnitureSystem/BP_FurnitureComponent.BP_FurnitureComponent_C|GetRequiresCutout (Actor|GetComponentbyClass _array_element "/Game/MastersProject/Core/FurnitureSystem/BP_FurnitureComponent.BP_FurnitureComponent_C"))
      (bind (_outhit _returnvalue) (Collision|LineTraceByChannel (+ (Transformation|GetActorLocation _array_element) (* (Math|Rotator|GetRotationXVector (Transformation|GetActorRotation _array_element)) 2e+02) "0.000000,0.000000,200.000000") (+ (Transformation|GetActorLocation _array_element) (* (Math|Rotator|GetRotationXVector (Transformation|GetActorRotation _array_element)) -2e+02) "0.000000,0.000000,200.000000") "TraceTypeQuery4" false 0 "ForDuration" false))
      (if _returnvalue
        (if (== (Components|GetOwner (.hitcomponent _outhit)) self)
          (bind _asstatic_mesh_component (Utilities|Casting|CastToStaticMeshComponent (.hitcomponent _outhit)))
          (Components|StaticMesh|SetStaticMesh _asstatic_mesh_component (Variables|/Game/MastersProject/Core/BuildingTools/PDA_RoomInfo.PDA_RoomInfo_C|GetDoorwayMesh (Variables|Default|GetRoomInfo)))
          (else
            (bind (_outhit_2 _returnvalue_2) (Collision|LineTraceByChannel (+ (Transformation|GetActorLocation _array_element) (* (Math|Rotator|GetRotationXVector (Transformation|GetActorRotation _array_element)) -2e+02) "0.000000,0.000000,200.000000") (+ (Transformation|GetActorLocation _array_element) (* (Math|Rotator|GetRotationXVector (Transformation|GetActorRotation _array_element)) 2e+02) "0.000000,0.000000,200.000000") "TraceTypeQuery4" false 0 "ForDuration" false))
            (if _returnvalue_2
              (if (== (Components|GetOwner (.hitcomponent _outhit_2)) self)
                (bind _asstatic_mesh_component_2 (Utilities|Casting|CastToStaticMeshComponent (.hitcomponent _outhit_2)))
                (Components|StaticMesh|SetStaticMesh _asstatic_mesh_component_2 (Variables|/Game/MastersProject/Core/BuildingTools/PDA_RoomInfo.PDA_RoomInfo_C|GetDoorwayMesh (Variables|Default|GetRoomInfo)))))))))))
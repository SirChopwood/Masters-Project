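; Test actor that procedurally builds a rectangular room from two corner points in its construction script, using Geometry Script dynamic meshes.
; Box-appended walls get rounded doorways cut by boolean subtraction of extruded rounded rectangles, one per Doors entry, each spawning a BP_BuildingNavMeshProxy child actor.
; Wall collision is generated from the carved mesh, and a box floor is added.
; Walls and floor receive dynamic materials with randomized hue and desaturation.
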(event EventBeginPlay)

(event Collision|EventActorBeginOverlap
  (params (OtherActor :type Actor%20Object%20Reference)))

(event EventTick
  (params (DeltaSeconds :type Float%20%28single-precision%29)))

(fn ConstructionScript
  (CallFunction|ReconstructRoomMeshes))

(fn ReconstructRoomMeshes
  (bind _corner1 (Variables|Default|GetCorner1))
  (bind _corner2 (Variables|Default|GetCorner2))
  (bind _corner1_2 (Variables|Default|GetCorner1))
  (bind _corner2_2 (Variables|Default|GetCorner2))
  (bind _returnvalue (AddComponent|AddDynamicMeshComponent false))
  (bind _output_get (Variables|Default|SetWallMeshComponent _returnvalue))
  (Collision|SetCollisionEnabled _output_get "QueryAndPhysics")
  (Collision|SetCollisionObjectType _output_get "ECC_WorldStatic")
  (Class|DynamicMeshComponent|EnableComplexasSimpleCollision _output_get)
  (bind _returnvalue_2 (DynamicMeshComponent|GetDynamicMesh _output_get))
  (Variables|Default|SetWallMesh _returnvalue_2)
  (Utilities|FlowControl|Sequence
    (:then_0
      ;[0.9544 1 0.4362] Calculate Room Dimensions
      (LocalVariables|SetRoomCenterPoint (Math|Vector|MakeVector (Math|Float|Lerp (.x _corner1) (.x _corner2) 0.5) (Math|Float|Lerp (.y _corner1) (.y _corner2) 0.5) 0.0))
      (LocalVariables|SetRoomExtents (Math|Vector|MakeVector (Math|Float|Absolute(Float) (- (.x _corner1) (.x _corner2))) (Math|Float|Absolute(Float) (- (.y _corner1) (.y _corner2))) 0.0)))
    (:then_1
      ;[0.523 1 0.5358] Generate Walls
      (Utilities|AddWall :CenterPoint (Math|Vector|MakeVector (.x (LocalVariables|GetRoomCenterPoint)) (.y _corner1_2) 0.0) :Length (.x (LocalVariables|GetRoomExtents)))
      (Utilities|AddWall :CenterPoint (Math|Vector|MakeVector (.x (LocalVariables|GetRoomCenterPoint)) (.y _corner2_2) 0.0) :Length (.x (LocalVariables|GetRoomExtents)))
      (Utilities|AddWall (Math|Vector|MakeVector (.x _corner2_2) (.y (LocalVariables|GetRoomCenterPoint)) 0.0) "0.000000,90.000000,0.000000" (.y (LocalVariables|GetRoomExtents)))
      (Utilities|AddWall (Math|Vector|MakeVector (.x _corner1_2) (.y (LocalVariables|GetRoomCenterPoint)) 0.0) "0.000000,90.000000,0.000000" (.y (LocalVariables|GetRoomExtents))))
    (:then_2
      ;[1 0.5298 0.212] Add Doors
      (bind _returnvalue_3 (AddComponent|AddDynamicMeshComponent false))
      (bind _returnvalue_4 (DynamicMeshComponent|GetDynamicMesh _returnvalue_3))
      (Variables|Default|SetToolMesh _returnvalue_4)
      (for _array_element (Variables|Default|GetDoors)
        (Utilities|AddDoor _array_element 1.5e+02 5e+01)))
    (:then_3
      ;[0.3926 0.9402 1] Apply Collision
      (Class|GeometryScriptLibraryCollisionFunctions|SetDynamicMeshCollisionfromMesh (Variables|Default|GetWallMesh) (Variables|Default|GetWallMeshComponent) (Utilities|Struct|MakeGeometryScriptCollisionfromMeshOptions true "MinVolumeShapes") 0))
    (:then_4
      ;[0.2916 0.3628 1] Add Floor
      (bind _returnvalue_5 (AddComponent|AddDynamicMeshComponent false))
      (bind _output_get_2 (Variables|Default|SetFloorMeshComponent _returnvalue_5))
      (bind _returnvalue_6 (DynamicMeshComponent|GetDynamicMesh _output_get_2))
      (bind _returnvalue_7 (Class|GeometryScriptLibraryMeshPrimitiveFunctions|AppendBox :TargetMesh _returnvalue_6 :Transform (Math|Transform|MakeTransform (Math|Vector|MakeVector (.x (LocalVariables|GetRoomCenterPoint)) (.y (LocalVariables|GetRoomCenterPoint)) 0.0) "0, 0, 0" "1.000000,1.000000,1.000000") :DimensionX (.x (LocalVariables|GetRoomExtents)) :DimensionY (.y (LocalVariables|GetRoomExtents)) :DimensionZ 2e+01 :Origin "Center" :Debug 0))
      (bind _selection (Class|GeometryScriptLibraryMeshSelectionFunctions|CreateSelectAllMeshSelection _returnvalue_7 "Vertices"))
      (Class|GeometryScriptLibraryMeshMaterialFunctions|SetMaterialIDforMeshSelection _returnvalue_7 _selection 0 false 0))
    (:then_5
      ;[1 0.3118 0.3416] Apply Materials
      ;;[1 1 1] Wall
      (bind _returnvalue_8 (Rendering|Material|CreateDynamicMaterialInstance "/Game/MastersProject/Core/BuildingTools/M_WallTest.M_WallTest" "None" "None" :!class /Script/Engine.KismetMaterialLibrary))
      (Rendering|Material|SetScalarParameterValue _returnvalue_8 "HueShift" (Math|Random|RandomFloatinRange 0.0 1.0) :!class /Script/Engine.MaterialInstanceDynamic)
      (GeometryScript|Scene|SetComponentMaterialList (Variables|Default|GetWallMeshComponent) (Utilities|Array|MakeArray _returnvalue_8) 0)
      ;;[1 1 1] Floor
      (bind _returnvalue_9 (Rendering|Material|CreateDynamicMaterialInstance "/Game/MastersProject/Core/BuildingTools/M_FloorTest.M_FloorTest" "None" "None" :!class /Script/Engine.KismetMaterialLibrary))
      (Rendering|Material|SetScalarParameterValue _returnvalue_9 "Desaturation" (Math|Random|RandomFloatinRange 0.5 -0.5) :!class /Script/Engine.MaterialInstanceDynamic)
      (GeometryScript|Scene|SetComponentMaterialList (Variables|Default|GetFloorMeshComponent) (Utilities|Array|MakeArray _returnvalue_9) 0))))
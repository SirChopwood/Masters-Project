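; BP_GameManager is a game manager that tracks active objectives and holds a list of placed furniture.
; InitManager stores the game mode and registers the manager on the player controller's BPFurniturePCComponent.
; Start and complete objective events add objective data assets uniquely to the active list and remove them.
; Tick prints the display name of every placed furniture each frame; nothing in these graphs fills that list.
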(event Custom|InitManager
  (params (GameMode :type GM%20Tavern%20Object%20Reference))
  (Variables|Default|SetGame%20Mode GameMode)
  (bind _aspc_player (Utilities|Casting|CastToPC_Player (Game|GetPlayerController 0)))
  (Variables|/Game/MastersProject/Core/FurnitureSystem/BP_FurniturePCComponent.BP_FurniturePCComponent_C|SetGameManager (Variables|/Game/MastersProject/Core/Characters/Player/PC_Player.PC_Player_C|GetBP_FurniturePCComponent _aspc_player) self))

(event EventTick
  (params (DeltaSeconds :type Float%20%28single-precision%29))
  (for _array_element (Variables|Default|GetPlacedFurnitures)
    (Development|PrintString (Utilities|GetDisplayName _array_element) true true "(R=0.000000,G=0.660000,B=1.000000,A=1.000000)" 0.0)))

(event EventIStartObjective
  (params (ObjectiveDataAsset :type Primary%20Data%20Asset%20Object%20Reference))
  (Utilities|Array|AddUnique (Variables|Default|GetActiveObjectives) ObjectiveDataAsset))

(event EventICompleteObjective
  (params (CompletedObjective :type Primary%20Data%20Asset%20Object%20Reference))
  (Utilities|Array|RemoveItem (Variables|Default|GetActiveObjectives) CompletedObjective))

(fn ConstructionScript)
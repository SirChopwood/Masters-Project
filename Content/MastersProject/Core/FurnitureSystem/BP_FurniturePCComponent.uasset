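; Player controller component for picking up, rotating and placing furniture actors that carry BP_FurnitureComponent2.
; Left click grabs or drops, R or middle mouse rotates by 90 degrees, and a looping timer lerps the held actor toward the cursor.
; Targets snap to a floor grid or, for Object types, the nearest tag-matched snap point.
; Room whitelist and blocker overlap checks drive the overlay material's validity without gating the drop.
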(event EventBeginPlay
  (bind _returnvalue (Rendering|Material|CreateDynamicMaterialInstance "/Game/MastersProject/Core/FurnitureSystem/M_PlacementOverlay.M_PlacementOverlay" "None" "None" :!class /Script/Engine.KismetMaterialLibrary))
  (Variables|Default|SetValidOverlayMaterial _returnvalue))

(event Input|MouseEvents|LeftMouseButton
  (params (Key :type Key%20Structure))
  (bind _returnvalue (Game|GetPlayerController 0))
  (bind _hitresult (Game|Player|GetHitResultUnderCursorbyChannel _returnvalue "TraceTypeQuery1" true))
  (bind _returnvalue_2 (Actor|GetComponentbyClass (.hitactor _hitresult) "/Game/MastersProject/Core/FurnitureSystem/BP_FurnitureComponent2.BP_FurnitureComponent2_C"))
  (:Pressed
    (Utilities|IsValid (Variables|Default|GetHeldActor)
      (:Is%20Valid
        (Utilities|Time|ClearandInvalidateTimerbyHandle (Variables|Default|GetHeldTimerRef))
        (for _array_element (Actor|GetComponentsByClass (Variables|Default|GetHeldActor) "/Script/Engine.MeshComponent")
          (Rendering|Material|SetOverlayMaterial _array_element 0 :!class /Script/Engine.MeshComponent))
        (Variables|Default|SetHeldActor 0)
        (Variables|Default|SetDesiredRotation "0, 0, 0"))
      (:Is%20Not%20Valid
        (Utilities|IsValid _returnvalue_2
          (:Is%20Valid
            (Variables|Default|SetHeldActor (.hitactor _hitresult))
            (Variables|Default|SetHeldComponent _returnvalue_2)
            (bind _returnvalue_3 (Utilities|Time|SetTimerbyFunctionName 0 "FurnitureMoveTick" 0.02 true))
            (Variables|Default|SetHeldTimerRef _returnvalue_3)
            (for _array_element_2 (Actor|GetComponentsByClass (Variables|Default|GetHeldActor) "/Script/Engine.MeshComponent")
              (Rendering|Material|SetOverlayMaterial _array_element_2 (Variables|Default|GetValidOverlayMaterial) :!class /Script/Engine.MeshComponent))))))))

(event Input|MouseEvents|MiddleMouseButton
  (params (Key :type Key%20Structure))
  (:Pressed
    (Variables|Default|SetDesiredRotation (Math|Rotator|CombineRotators (Variables|Default|GetDesiredRotation) "0.000000,90.000000,0.000000"))))

(event Input|KeyboardEvents|R
  (params (Key :type Key%20Structure))
  (:Pressed
    (Variables|Default|SetDesiredRotation (Math|Rotator|CombineRotators (Variables|Default|GetDesiredRotation) "0.000000,90.000000,0.000000"))))

(fn FurnitureMoveTick
  (bind _result (Utilities|GetMouseLocation))
  (bind _result_2 (Utilities|GetMouseLocation))
  (bind _returnvalue (Class|KismetMathLibrary|VectorSnappedtoGrid _result 1e+02))
  (bind _returnvalue_2 (Class|KismetMathLibrary|VectorSnappedtoGrid _result_2 1e+02))
  (bind (_x _y) (Math|Vector|BreakVector _returnvalue))
  (switch Utilities|FlowControl|Switch|SwitchonE_FurnitureSnappingType (Variables|/Game/MastersProject/Core/FurnitureSystem/BP_FurnitureComponent2.BP_FurnitureComponent2_C|GetSnapType (Variables|Default|GetHeldComponent))
    (:NewEnumerator0
      ;[1 0.6555 0.2458] Floor Snapping
      (CallFunction|UpdateHeldActorTransform (Math|Vector|MakeVector _x _y 0.0) (Variables|Default|GetDesiredRotation)))
    (:NewEnumerator2
      ;[0.2187 0.4422 1] Object Snapping
      (bind _outhits (Collision|MultiSphereTraceByChannel _result_2 _result_2 1.2e+03 "TraceTypeQuery1" false 0 "ForDuration" true "(R=1.000000,G=0.487687,B=0.000000,A=1.000000)" "(R=1.000000,G=0.264881,B=0.000000,A=1.000000)" 0.02))
      (for _array_element _outhits
        ;;[0.7397 1 0.2397] Find Nearest Snap Point
        (Utilities|IsValid (Actor|GetComponentbyClass (.hitactor _array_element) "/Game/MastersProject/Core/FurnitureSystem/BP_FurnitureComponent2.BP_FurnitureComponent2_C")
          (:Is%20Valid
            (for (_array_element_2 _array_index) (Variables|/Game/MastersProject/Core/FurnitureSystem/BP_FurnitureComponent2.BP_FurnitureComponent2_C|GetSnapPoints (Actor|GetComponentbyClass (.hitactor _array_element) "/Game/MastersProject/Core/FurnitureSystem/BP_FurnitureComponent2.BP_FurnitureComponent2_C"))
              (if (Utilities|Enum|Equal(Enum) (Variables|/Game/MastersProject/Core/FurnitureSystem/BP_FurnitureComponent2.BP_FurnitureComponent2_C|GetSnapTag (Variables|Default|GetHeldComponent)) (.whitelisttag _array_element_2))
                (Rendering|Debug|DrawDebugSphere (+ (Math|Vector|RotateVectorAroundAxis (.location _array_element_2) (.yaw (Transformation|GetActorRotation (.hitactor _array_element))) "0.000000,0.000000,1.000000") (Transformation|GetActorLocation (.hitactor _array_element))) 3e+01 12 "(R=1.000000,G=1.000000,B=1.000000,A=1.000000)" 0.02 2e+01)
                (if (< (Math|Vector|Distance(Vector) _result_2 (+ (Math|Vector|RotateVectorAroundAxis (.location _array_element_2) (.yaw (Transformation|GetActorRotation (.hitactor _array_element))) "0.000000,0.000000,1.000000") (Transformation|GetActorLocation (.hitactor _array_element)))) (LocalVariables|GetNearestSnapPointDistance))
                  (LocalVariables|SetNearestSnapPointDistance (Math|Vector|Distance(Vector) _result_2 (+ (Math|Vector|RotateVectorAroundAxis (.location _array_element_2) (.yaw (Transformation|GetActorRotation (.hitactor _array_element))) "0.000000,0.000000,1.000000") (Transformation|GetActorLocation (.hitactor _array_element)))))
                  (LocalVariables|SetNearestSnapPointIndex _array_index)
                  (LocalVariables|SetNearestSnapPointActor (.hitactor _array_element))
                  (LocalVariables|SetNearestSnapPointComponent (Actor|GetComponentbyClass (.hitactor _array_element) "/Game/MastersProject/Core/FurnitureSystem/BP_FurnitureComponent2.BP_FurnitureComponent2_C"))))))))
      (Utilities|IsValid (LocalVariables|GetNearestSnapPointActor)
        (:Is%20Valid
          ;;[0.3345 1 0.4445] Snap To Snap Point
          (CallFunction|UpdateHeldActorTransform (+ (Transformation|GetActorLocation (LocalVariables|GetNearestSnapPointActor)) (Math|Vector|RotateVectorAroundAxis (.location (Utilities|Array|Get(acopy) (Variables|/Game/MastersProject/Core/FurnitureSystem/BP_FurnitureComponent2.BP_FurnitureComponent2_C|GetSnapPoints (LocalVariables|GetNearestSnapPointComponent)) (LocalVariables|GetNearestSnapPointIndex))) (.yaw (Transformation|GetActorRotation (LocalVariables|GetNearestSnapPointActor))) "0.000000,0.000000,1.000000")) (Math|Rotator|CombineRotators (Math|Rotator|MakeRotator (.roll (Transformation|GetActorRotation (LocalVariables|GetNearestSnapPointActor))) (.pitch (Transformation|GetActorRotation (LocalVariables|GetNearestSnapPointActor))) (.yaw (Transformation|GetActorRotation (LocalVariables|GetNearestSnapPointActor)))) (.rotation (Utilities|Array|Get(acopy) (Variables|/Game/MastersProject/Core/FurnitureSystem/BP_FurnitureComponent2.BP_FurnitureComponent2_C|GetSnapPoints (LocalVariables|GetNearestSnapPointComponent)) (LocalVariables|GetNearestSnapPointIndex))))))
        (:Is%20Not%20Valid
          ;;[0.2619 1 0.8901] No Snap, Track Cursor
          (CallFunction|UpdateHeldActorTransform (Math|Vector|MakeVector (.x _returnvalue_2) (.y _returnvalue_2) 0.0) (Variables|Default|GetDesiredRotation)))))))

(fn FurnitureMoveValidCheck
  (params (Component%20Transform%20Location :type Vector) (Component%20Transform%20Rotation :type Rotator))
  (bind _heldactor (Variables|Default|GetHeldActor))
  (bind _returnvalue (Transformation|GetActorLocation _heldactor))
  (Utilities|FlowControl|Sequence
    (:then_0
      ;[1 1 1] Whitelist Check
      (bind _outhit (Collision|LineTraceByChannel _returnvalue (+ _returnvalue "0.000000,0.000000,1.000000") "TraceTypeQuery3" false 0 "None"))
      (bind _asbp_room_generator (Utilities|Casting|CastToBP_RoomGenerator (.hitactor _outhit)))
      (LocalVariables|SetWhitelistCheck (Utilities|Array|ContainsItem (Variables|/Game/MastersProject/Core/FurnitureSystem/BP_FurnitureComponent2.BP_FurnitureComponent2_C|GetRoomWhitelist (Variables|Default|GetHeldComponent)) (Variables|/Game/MastersProject/Core/BuildingTools/BP_RoomGenerator.BP_RoomGenerator_C|GetRoomInfo _asbp_room_generator))))
    (:then_1
      ;[1 1 1] BlockerCheck
      (for _array_element (Actor|GetComponentsByClass (Variables|Default|GetHeldActor) "/Script/Engine.PrimitiveComponent")
        (bind _outcomponents (Class|KismetSystemLibrary|ComponentOverlapComponents _array_element (Math|Transform|MakeTransform Component%20Transform%20Location Component%20Transform%20Rotation "1.000000,1.000000,1.000000") (Utilities|Array|MakeArray "ObjectTypeQuery7")))
        (for _array_element_2 _outcomponents
          (if (Utilities|Enum|Equal(Enum) (Collision|GetCollisionResponsetoChannel _array_element_2 "ECC_GameTraceChannel3") "ECR_Block")
            (LocalVariables|SetBlockerCheck false)))))
    (:then_2
      (Rendering|Material|SetScalarParameterValue (Variables|Default|GetValidOverlayMaterial) "Valid" (Math|Conversions|ToFloat(Boolean) (and (LocalVariables|GetWhitelistCheck) (LocalVariables|GetBlockerCheck))) :!class /Script/Engine.MaterialInstanceDynamic)
      (return (and (LocalVariables|GetWhitelistCheck) (LocalVariables|GetBlockerCheck))))))

(fn UpdateHeldActorTransform
  (params (Location :type Vector) (Rotation :type Rotator))
  (bind _heldactor (Variables|Default|GetHeldActor))
  (Transformation|SetActorLocation _heldactor (Math|Vector|Lerp(Vector) (Transformation|GetActorLocation _heldactor) Location 0.2) false false)
  (Transformation|SetActorRotation _heldactor (Math|Rotator|Lerp(Rotator) (Transformation|GetActorRotation _heldactor) Rotation 0.2 true))
  (CallFunction|FurnitureMoveValidCheck Location Rotation)
  (return))
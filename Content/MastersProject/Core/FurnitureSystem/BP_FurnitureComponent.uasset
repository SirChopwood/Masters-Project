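; BP_FurnitureComponent is a furniture component that gives its owning actor a companion BP_BuildingNavMeshProxy actor.
; On BeginPlay, if AddNavMeshProxy is set, it spawns the proxy at the owner's location with a rotation offset and enlarged scale, storing the reference.
; UpdateNavMeshProxy destroys the stored proxy and respawns it from the owner's current transform.
; Each spawn prints the proxy's name and the world's total proxy count as debug output.
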(event Custom|UpdateNavMeshProxy
  (bind _returnvalue (Components|GetOwner))
  (bind _returnvalue_2 (Transformation|GetActorTransform _returnvalue))
  (Actor|DestroyActor (Variables|Default|GetNavMeshProxy))
  (bind _returnvalue_3 (Game|SpawnActorfromClass "/Game/MastersProject/Core/BuildingTools/BP_BuildingNavMeshProxy.BP_BuildingNavMeshProxy_C" (Math|Transform|MakeTransform (.location _returnvalue_2) (Math|Rotator|CombineRotators (.rotation _returnvalue_2) "0.000000,90.000000,0.000000") "5.000000,5.000000,5.000000") "AlwaysSpawn" "MultiplyWithRoot" 0 0))
  (bind _output_get (Variables|Default|SetNavMeshProxy _returnvalue_3))
  (Development|PrintString (Utilities|GetDisplayName _output_get))
  (bind _outactors (Actor|GetAllActorsOfClass "/Game/MastersProject/Core/BuildingTools/BP_BuildingNavMeshProxy.BP_BuildingNavMeshProxy_C"))
  (Development|PrintString (Utilities|String|ToString(Integer) (Utilities|Array|Length _outactors))))

(event EventBeginPlay
  (bind _returnvalue (Components|GetOwner))
  (bind _returnvalue_2 (Transformation|GetActorTransform _returnvalue))
  (if (Variables|FURNITURE-WallSnapping|GetAddNavMeshProxy)
    (bind _returnvalue_3 (Game|SpawnActorfromClass "/Game/MastersProject/Core/BuildingTools/BP_BuildingNavMeshProxy.BP_BuildingNavMeshProxy_C" (Math|Transform|MakeTransform (.location _returnvalue_2) (Math|Rotator|CombineRotators (.rotation _returnvalue_2) "0.000000,90.000000,0.000000") "5.000000,5.000000,5.000000") "AlwaysSpawn" "MultiplyWithRoot" 0 0))
    (bind _output_get (Variables|Default|SetNavMeshProxy _returnvalue_3))
    (Development|PrintString (Utilities|GetDisplayName _output_get))
    (bind _outactors (Actor|GetAllActorsOfClass "/Game/MastersProject/Core/BuildingTools/BP_BuildingNavMeshProxy.BP_BuildingNavMeshProxy_C"))
    (Development|PrintString (Utilities|String|ToString(Integer) (Utilities|Array|Length _outactors)))))
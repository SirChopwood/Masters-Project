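; BP_TestDoor is a test door in the furniture system that opens automatically while customers are near it.
; Its Sphere overlap events add actors of exactly class BP_Customer to UserList and remove actors as they leave.
; After each change, UpdateDoorState snaps DoorHinge open a quarter turn if the list has any users, or closed if empty, with no animation.
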(event OnComponentBeginOverlap(Sphere)
  (params (OverlappedComponent :type Primitive%20Component%20Object%20Reference) (OtherActor :type Actor%20Object%20Reference) (OtherComp :type Primitive%20Component%20Object%20Reference) (OtherBodyIndex :type Integer) (bFromSweep :type Boolean) (SweepResult :type Hit%20Result%20Structure%20%28by%20ref%29))
  (if (== (Utilities|GetClass OtherActor) "/Game/MastersProject/Core/Characters/Customer/BP_Customer.BP_Customer_C")
    (Utilities|Array|AddUnique (Variables|Default|GetUserList) OtherActor)
    (CallFunction|UpdateDoorState)))

(event OnComponentEndOverlap(Sphere)
  (params (OverlappedComponent :type Primitive%20Component%20Object%20Reference) (OtherActor :type Actor%20Object%20Reference) (OtherComp :type Primitive%20Component%20Object%20Reference) (OtherBodyIndex :type Integer))
  (Utilities|Array|RemoveItem (Variables|Default|GetUserList) OtherActor)
  (CallFunction|UpdateDoorState))

(event Custom|UpdateDoorState
  (bind _doorhinge (Variables|Default|GetDoorHinge))
  (if (> (Utilities|Array|Length (Variables|Default|GetUserList)) 0)
    (Transformation|SetRelativeRotation _doorhinge "0.000000,90.000000,0.000000" false false)
    (else
      (Transformation|SetRelativeRotation _doorhinge "0, 0, 0" false false))))

(fn ConstructionScript)
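; Delivery zone actor for the furniture system that handles item purchases and spawns the bought furniture inside its box.
; On BeginPlay it caches the currency component from the game mode and the furniture component from player controller 0.
; PurchaseItem spends the price read from the furniture class defaults.
; If payment succeeds, it spawns the item at a random XY within the box bounds and notifies the controller component.
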(event Custom|PurchaseItem
  (params (FurnitureInfo :type BP%20F%20Master%20Class%20Reference))
  (bind _box (Variables|Default|GetBox))
  (bind (_origin _boxextent) (Collision|GetComponentBounds _box))
  (bind _returnvalue (Math|Random|RandomPointinBoundingBox _origin _boxextent))
  (bind _success (Default|SpendCurrency (Variables|Default|GetCurrencyComponent) (Utilities|GetClassDefaults FurnitureInfo) "NewEnumerator0"))
  (if _success
    (bind _returnvalue_2 (Game|SpawnActorfromClass FurnitureInfo (Math|Transform|MakeTransform (Math|Vector|MakeVector (.x _returnvalue) (.y _returnvalue) 0.0) "0, 0, 0" "1.000000,1.000000,1.000000") "Undefined" "MultiplyWithRoot" 0 0))
    (Default|CallOnFurniturePurchase (Variables|Default|GetFurniturePCComponent) _returnvalue_2)))

(event EventBeginPlay
  (Variables|Default|SetCurrencyComponent (Actor|GetComponentbyClass (Game|GetGameMode) "/Game/MastersProject/Core/AC_Currency.AC_Currency_C"))
  (Variables|Default|SetFurniturePCComponent (Actor|GetComponentbyClass (Game|GetPlayerController 0) "/Game/MastersProject/Core/FurnitureSystem/BP_FurniturePCComponent.BP_FurniturePCComponent_C")))

(fn ConstructionScript)
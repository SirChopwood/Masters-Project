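; BP_AI_Spawner is an actor that spawns a limited number of BP_Customer characters around its location.
; BeginPlay starts a looping timer at the spawn delay to drive spawning.
; The Spawn event places each customer at a random reachable navmesh point within the radius and clears the timer once the maximum count is reached.
; The construction script draws a debug sphere showing the spawn radius.
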(event Custom|Spawn
  (if (< (Variables|Default|GetCurrentNumber) (Variables|Config|GetMaxNumberToSpawn))
    (Game|SpawnActorfromClass "/Game/MastersProject/Core/Characters/Customer/BP_Customer.BP_Customer_C" (Math|Transform|MakeTransform (.RandomLocation (AI|Navigation|GetRandomReachablePointinRadius (Transformation|GetActorLocation) (Variables|Config|GetRadius) 0 0)) "0, 0, 0" "1.000000,1.000000,1.000000") "AdjustIfPossibleButAlwaysSpawn" "MultiplyWithRoot" 0 0)
    (Math|Integer|IncrementInt (Variables|Default|GetCurrentNumber))
    (else
      (Utilities|Time|ClearandInvalidateTimerbyHandle (Variables|Default|GetSpawnHandle)))))

(event EventBeginPlay
  (bind _returnvalue (Utilities|Time|SetTimerbyEvent (EventDispatchers|CreateEvent :!event Custom|Spawn) (Variables|Config|GetSpawnDelay) true))
  (Variables|Default|SetSpawnHandle _returnvalue))

(fn ConstructionScript
  (Rendering|Debug|DrawDebugSphere (Transformation|GetActorLocation) (Variables|Config|GetRadius) 12 "(R=0.000000,G=0.000000,B=0.000000,A=1.000000)" 0.0 2.0))
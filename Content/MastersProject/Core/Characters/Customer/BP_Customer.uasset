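; AI guild customer that rolls a random name, weighted needs and skills, then decays hunger, tiredness, fellowship and willpower on looping timers mirrored to the Blackboard.
; Finds nearby matching furniture, preferring unused over not full; regenerating pauses that need's decay until full.
; Leaves unsuccessfully when three needs empty, or successfully after a regen if average needs reach the happy threshold, paying its skill total.
; Also provides an NPC stats inspector window.
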(event Custom|HungerTimer
  ;[1 1 1] Hunger Timer
  (CallFunction|UpdateNeedVariable (Variables|Needs|Basic|GetHunger) "NewEnumerator0" (Variables|Config|Stats|GetMaxHunger) (Variables|Config|Stats|GetDecreaseValue) "Hunger"))

(event Custom|SleepTimer
  ;[1 1 1] Sleep Timer
  (CallFunction|UpdateNeedVariable (Variables|Needs|Basic|GetTiredness) "NewEnumerator1" (Variables|Config|Stats|GetMaxTiredness) (Variables|Config|Stats|GetDecreaseValue) "Tiredness"))

(event Custom|StartRegen
  (params (Task :type E_Tasks%20Enum :default "NewEnumerator3") (RegenRate :type Float%20%28double-precision%29) (RegenValue :type Float%20%28double-precision%29))
  ;[1 1 1] Start Regen
  (Variables|Default|SetRegenRate RegenRate)
  (Variables|Default|SetRegenValue RegenValue)
  (Variables|Default|SetTaskToRegen Task)
  (Utilities|FlowControl|Sequence
    (:then_0
      (bind _returnvalue (Utilities|Time|SetTimerbyFunctionName 0 "RegenNeedValue" (Variables|Default|GetRegenRate) true))
      (Variables|TimerHandles|SetRegenHandle _returnvalue)
      (Animation|Montage|PlayMontage (Variables|Character|GetMesh) (Utilities|Select :Index (Variables|Default|GetTaskToRegen) :NewEnumerator3 0 :NewEnumerator0 "/Game/MastersProject/Characters/Barbarian/Barbarian_AM.Barbarian_AM" :NewEnumerator1 0 :NewEnumerator4 0 :NewEnumerator5 0 :NewEnumerator6 0 :NewEnumerator7 0 :NewEnumerator8 0 :NewEnumerator9 0)))
    (:then_1
      (Utilities|Time|PauseTimerbyHandle (Utilities|Select :Index (Variables|Default|GetTaskToRegen) :NewEnumerator3 "" :NewEnumerator0 (Variables|TimerHandles|GetHungerHandle) :NewEnumerator1 (Variables|TimerHandles|GetTiredHandle) :NewEnumerator4 (Variables|TimerHandles|GetFellowshipHandle) :NewEnumerator5 (Variables|TimerHandles|GetWillpowerHandle) :NewEnumerator6 "" :NewEnumerator7 "" :NewEnumerator8 "" :NewEnumerator9 "")))))

(event Custom|FellowshipTimer
  ;[1 1 1] Fellowship Timer
  (CallFunction|UpdateNeedVariable (Variables|Needs|Basic|GetFellowship) "NewEnumerator4" (Variables|Config|Stats|GetMaxFellowship) (Variables|Config|Stats|GetDecreaseValue) "Fellowship"))

(event Custom|WillpowerTimer
  ;[1 1 1] Willpower Timer
  (CallFunction|UpdateNeedVariable (Variables|Needs|Basic|GetWillpower) "NewEnumerator5" (Variables|Config|Stats|GetMaxWillpower) (Variables|Config|Stats|GetDecreaseValue) "Willpower"))

(event Custom|Init
  (params (GameMode :type GM%20Tavern%20Object%20Reference))
  ;[1 1 1] Start Hunger and Sleep Timers
  (Variables|Default|SetGameMode GameMode)
  (CallFunction|RollNeedValues)
  (CallFunction|SetDecreaseRates/Values)
  (CallFunction|SetNeedTimers)
  (CallFunction|SetCustomerName))

(event EventISetQueueIndex
  (params (NewIndex :type Integer))
  ;[1 1 1] Set Queue Index
  (Class|BlackboardComponent|SetValueasInt (AI|GetBlackboard (AI|GetAIController self)) (Utilities|Name|MakeLiteralName "QueueIndex") NewIndex))

(fn ConstructionScript)

(fn UpdateNeedVariable
  (params (Need :type Float%20%28double-precision%29%20%28by%20ref%29) (NeedTask :type E_Tasks%20Enum :default "NewEnumerator3") (MaxNeed :type Float%20%28double-precision%29) (Change :type Float%20%28double-precision%29) (KeyName :type Name))
  (bind _returnvalue (+ Need Change))
  (bind _returnvalue_2 (Math|Float|Clamp(Float) _returnvalue 0.0 MaxNeed))
  (|SetBy-RefVar Need _returnvalue_2)
  (AI|Components|Blackboard|SetValueasFloat (AI|GetBlackboard 0) KeyName (/ Need MaxNeed))
  (bind _3_4empty_ (CallFunction|EmptyNeedCheck NeedTask (== _returnvalue_2 0.0)))
  (if _3_4empty_
    (Default|CallOnLeaveGuild self false 0.0)
    (for _array_element (Utilities|Array|MakeArray (Variables|TimerHandles|GetHungerHandle) (Variables|TimerHandles|GetTiredHandle) (Variables|TimerHandles|GetFellowshipHandle) (Variables|TimerHandles|GetWillpowerHandle))
      (Utilities|Time|ClearandInvalidateTimerbyHandle _array_element))
    (return false)
    (else
      (return (>= Need MaxNeed)))))

(fn GetClosestObject
  (params (Task :type E_Tasks%20Enum :default "NewEnumerator3"))
  (bind _gamemode (Variables|Default|GetGameMode))
  (bind _gamemanager (Variables|/Game/MastersProject/Core/GM_Tavern.GM_Tavern_C|GetGameManager _gamemode))
  (bind _placedfurnitures (Variables|/Game/MastersProject/Core/BP_GameManager.BP_GameManager_C|GetPlacedFurnitures _gamemanager))
  (Utilities|Array|Clear (Variables|Default|GetValidObjects))
  (Utilities|IsValid _gamemanager
    (:Is%20Valid
      (if (> (Utilities|Array|Length _placedfurnitures) 0)
        (for _array_element _placedfurnitures
          (Utilities|IsValid (Actor|GetComponentbyClass _array_element "/Game/MastersProject/Core/FurnitureSystem/SC_FurnitureNeedComponent.SC_FurnitureNeedComponent_C")
            (:Is%20Valid
              (if (Utilities|Enum|Equal(Enum) (Variables|/Game/MastersProject/Core/FurnitureSystem/SC_FurnitureNeedComponent.SC_FurnitureNeedComponent_C|GetNeedToFulffill (Actor|GetComponentbyClass _array_element "/Game/MastersProject/Core/FurnitureSystem/SC_FurnitureNeedComponent.SC_FurnitureNeedComponent_C")) Task)
                (Utilities|Array|AddUnique (Variables|Default|GetValidObjects) _array_element)))))
        (CallFunction|SortObjectsbyDistance)
        (for _array_element_2 (Variables|Default|GetValidObjects)
          (if (not (Variables|/Game/MastersProject/Core/FurnitureSystem/SC_FurnitureNeedComponent.SC_FurnitureNeedComponent_C|GetIsBeingUsed? (Actor|GetComponentbyClass _array_element_2 "/Game/MastersProject/Core/FurnitureSystem/SC_FurnitureNeedComponent.SC_FurnitureNeedComponent_C")))
            (return _array_element_2 true)))
        (for _array_element_3 (Variables|Default|GetValidObjects)
          (if (not (Variables|/Game/MastersProject/Core/FurnitureSystem/SC_FurnitureNeedComponent.SC_FurnitureNeedComponent_C|GetIsFull? (Actor|GetComponentbyClass _array_element_3 "/Game/MastersProject/Core/FurnitureSystem/SC_FurnitureNeedComponent.SC_FurnitureNeedComponent_C")))
            (return _array_element_3 true)))
        (return 0 false)
        (else
          (return 0 false))))
    (:Is%20Not%20Valid
      (return 0 false))))

(fn SortObjectsbyDistance
  (bind _validobjects (Variables|Default|GetValidObjects))
  (for (_array_element _array_index) _validobjects
    (for _index (range _array_index (- (Utilities|Array|Length _validobjects) 1))
      (if (< (Transformation|GetDistanceTo (Utilities|Array|Get(acopy) (Variables|Default|GetValidObjects) _index) self) (Transformation|GetDistanceTo _array_element self))
        (Utilities|Array|Swap (Variables|Default|GetValidObjects) _array_index _index))))
  (return))

(fn ClearValidObjects
  (Utilities|Array|Clear (Variables|Default|GetValidObjects)))

(fn SetStartingNeeds
  (for (_array_element _array_index) (Variables|Config|Stats|GetNeedWeighting)
    (switch Utilities|FlowControl|Switch|SwitchonE_Tasks _array_element
      (:NewEnumerator0
        (Variables|Needs|Basic|SetHunger (Math|Conversions|ToFloat(Integer) (Math|Float|Floor (* (Utilities|Select :Index _array_element :NewEnumerator3 0.0 :NewEnumerator0 (Variables|Config|Stats|GetMaxHunger) :NewEnumerator1 (Variables|Config|Stats|GetMaxTiredness) :NewEnumerator4 (Variables|Config|Stats|GetMaxFellowship) :NewEnumerator5 (Variables|Config|Stats|GetMaxWillpower) :NewEnumerator6 0.0 :NewEnumerator7 0.0 :NewEnumerator8 0.0 :NewEnumerator9 0.0) (Utilities|Array|Get(acopy) (Variables|Default|GetAlphas) _array_index))))))
      (:NewEnumerator1
        (Variables|Needs|Basic|SetTiredness (Math|Conversions|ToFloat(Integer) (Math|Float|Floor (* (Utilities|Select :Index _array_element :NewEnumerator3 0.0 :NewEnumerator0 (Variables|Config|Stats|GetMaxHunger) :NewEnumerator1 (Variables|Config|Stats|GetMaxTiredness) :NewEnumerator4 (Variables|Config|Stats|GetMaxFellowship) :NewEnumerator5 (Variables|Config|Stats|GetMaxWillpower) :NewEnumerator6 0.0 :NewEnumerator7 0.0 :NewEnumerator8 0.0 :NewEnumerator9 0.0) (Utilities|Array|Get(acopy) (Variables|Default|GetAlphas) _array_index))))))
      (:NewEnumerator4
        (Variables|Needs|Basic|SetFellowship (Math|Conversions|ToFloat(Integer) (Math|Float|Floor (* (Utilities|Select :Index _array_element :NewEnumerator3 0.0 :NewEnumerator0 (Variables|Config|Stats|GetMaxHunger) :NewEnumerator1 (Variables|Config|Stats|GetMaxTiredness) :NewEnumerator4 (Variables|Config|Stats|GetMaxFellowship) :NewEnumerator5 (Variables|Config|Stats|GetMaxWillpower) :NewEnumerator6 0.0 :NewEnumerator7 0.0 :NewEnumerator8 0.0 :NewEnumerator9 0.0) (Utilities|Array|Get(acopy) (Variables|Default|GetAlphas) _array_index))))))
      (:NewEnumerator5
        (Variables|Needs|Basic|SetWillpower (Math|Conversions|ToFloat(Integer) (Math|Float|Floor (* (Utilities|Select :Index _array_element :NewEnumerator3 0.0 :NewEnumerator0 (Variables|Config|Stats|GetMaxHunger) :NewEnumerator1 (Variables|Config|Stats|GetMaxTiredness) :NewEnumerator4 (Variables|Config|Stats|GetMaxFellowship) :NewEnumerator5 (Variables|Config|Stats|GetMaxWillpower) :NewEnumerator6 0.0 :NewEnumerator7 0.0 :NewEnumerator8 0.0 :NewEnumerator9 0.0) (Utilities|Array|Get(acopy) (Variables|Default|GetAlphas) _array_index))))))))
  (return))

(fn SetNeedTimers
  (bind _returnvalue (Utilities|Time|SetTimerbyEvent (EventDispatchers|CreateEvent :!event Custom|HungerTimer) (Variables|DecreaseRates|GetHungerDecreaseRate) true))
  (Variables|TimerHandles|SetHungerHandle _returnvalue)
  (bind _returnvalue_2 (Utilities|Time|SetTimerbyEvent (EventDispatchers|CreateEvent :!event Custom|SleepTimer) (Variables|DecreaseRates|GetSleepDecreaseRate) true))
  (Variables|TimerHandles|SetTiredHandle _returnvalue_2)
  (bind _returnvalue_3 (Utilities|Time|SetTimerbyEvent (EventDispatchers|CreateEvent :!event Custom|FellowshipTimer) (Variables|DecreaseRates|GetFellowDecreaseRate) true))
  (Variables|TimerHandles|SetFellowshipHandle _returnvalue_3)
  (bind _returnvalue_4 (Utilities|Time|SetTimerbyEvent (EventDispatchers|CreateEvent :!event Custom|WillpowerTimer) (Variables|DecreaseRates|GetWillDecreaseRate) true))
  (Variables|TimerHandles|SetWillpowerHandle _returnvalue_4)
  (return))

(fn RollNeedValues
  ;[1 1 1] Roll Random Alphas
  (for _index (range 0 (- (Utilities|Array|Length (Variables|Config|Stats|GetNeedWeighting)) 1))
    (Utilities|Array|Add (Variables|Default|GetAlphas) (Math|Random|RandomFloatinRange 0.5 0.8)))
  (CallFunction|OrderNeedValues)
  (CallFunction|SetStartingNeeds)
  (CallFunction|SetStartingSkills)
  (return))

(fn OrderNeedValues
  (bind _alphas (Variables|Default|GetAlphas))
  ;[1 1 1] Order Alphas
  (for (_array_element _array_index) _alphas
    (for _index (range _array_index (- (Utilities|Array|Length _alphas) 1))
      (if (> (Utilities|Array|Get(acopy) (Variables|Default|GetAlphas) _index) _array_element)
        (Utilities|Array|Swap (Variables|Default|GetAlphas) _array_index _index))))
  (return))

(fn RegenNeedValue
  (bind _isfull_ (CallFunction|UpdateNeedVariable (Utilities|Select :Index (Variables|Default|GetTaskToRegen) :NewEnumerator3 0.0 :NewEnumerator0 (Variables|Needs|Basic|GetHunger) :NewEnumerator1 (Variables|Needs|Basic|GetTiredness) :NewEnumerator4 (Variables|Needs|Basic|GetFellowship) :NewEnumerator5 (Variables|Needs|Basic|GetWillpower) :NewEnumerator6 0.0 :NewEnumerator7 0.0 :NewEnumerator8 0.0 :NewEnumerator9 0.0) (Variables|Default|GetTaskToRegen) (Utilities|Select :Index (Variables|Default|GetTaskToRegen) :NewEnumerator3 0.0 :NewEnumerator0 (Variables|Config|Stats|GetMaxHunger) :NewEnumerator1 (Variables|Config|Stats|GetMaxTiredness) :NewEnumerator4 (Variables|Config|Stats|GetMaxFellowship) :NewEnumerator5 (Variables|Config|Stats|GetMaxWillpower) :NewEnumerator6 0.0 :NewEnumerator7 0.0 :NewEnumerator8 0.0 :NewEnumerator9 0.0) (Variables|Default|GetRegenValue) (Utilities|Select :Index (Variables|Default|GetTaskToRegen) :NewEnumerator3 "None" :NewEnumerator0 "Hunger" :NewEnumerator1 "Tiredness" :NewEnumerator4 "Fellowship" :NewEnumerator5 "Willpower" :NewEnumerator6 "None" :NewEnumerator7 "None" :NewEnumerator8 "None" :NewEnumerator9 "None")))
  (if _isfull_
    (Utilities|Time|UnpauseTimerbyHandle (Utilities|Select :Index (Variables|Default|GetTaskToRegen) :NewEnumerator3 "" :NewEnumerator0 (Variables|TimerHandles|GetHungerHandle) :NewEnumerator1 (Variables|TimerHandles|GetTiredHandle) :NewEnumerator4 (Variables|TimerHandles|GetFellowshipHandle) :NewEnumerator5 (Variables|TimerHandles|GetWillpowerHandle) :NewEnumerator6 "" :NewEnumerator7 "" :NewEnumerator8 "" :NewEnumerator9 ""))
    (CallFunction|StopRegen)))

(fn StopRegen
  (Utilities|Time|ClearandInvalidateTimerbyHandle (Variables|TimerHandles|GetRegenHandle))
  (bind _asactor (Utilities|Casting|CastToActor (AI|Components|Blackboard|GetValueasObject (AI|GetBlackboard 0) (Utilities|Name|MakeLiteralName "TargetObject")))
    (:then
      (Default|StopInteracting (Actor|GetComponentbyClass _asactor "/Game/MastersProject/Core/FurnitureSystem/SC_FurnitureNeedComponent.SC_FurnitureNeedComponent_C") self)
      (AI|Components|Blackboard|SetValueasObject (AI|GetBlackboard 0) (Utilities|Name|MakeLiteralName "TargetObject") 0)
      (AI|Components|Blackboard|SetValueasEnum (AI|GetBlackboard 0) (Utilities|Name|MakeLiteralName "CurrentTask") (Utilities|Enum|LiteralenumE_Tasks "NewEnumerator3"))
      (Variables|Default|SetTaskToRegen "NewEnumerator3")
      (Default|CallOnStoppedRegen)
      (Animation|StopAnimMontage (Animation|GetCurrentMontage :!class /Script/Engine.Character))
      (if (>= (/ (+ (Variables|Needs|Basic|GetHunger) (Variables|Needs|Basic|GetTiredness) (Variables|Needs|Basic|GetWillpower) (Variables|Needs|Basic|GetFellowship)) 4.0) (* (/ (+ (Variables|Config|Stats|GetMaxHunger) (Variables|Config|Stats|GetMaxTiredness) (Variables|Config|Stats|GetMaxFellowship) (Variables|Config|Stats|GetMaxWillpower)) 4.0) (Variables|Config|Stats|GetHappyPercentage)))
        (Default|CallOnLeaveGuild self true (+ (Variables|Needs|Combat|GetToughness) (Variables|Needs|Combat|GetWeaponSkill) (Variables|Needs|Combat|GetEquipment) (Variables|Needs|Combat|GetSpellCraft)))
        (for _array_element (Utilities|Array|MakeArray (Variables|TimerHandles|GetHungerHandle) (Variables|TimerHandles|GetTiredHandle) (Variables|TimerHandles|GetFellowshipHandle) (Variables|TimerHandles|GetWillpowerHandle))
          (Utilities|Time|ClearandInvalidateTimerbyHandle _array_element))
        (return)
        (else
          (return))))
    (:CastFailed
      (return))))

(fn SetDecreaseRates/Values
  (bind _needweighting (Variables|Config|Stats|GetNeedWeighting))
  (for (_array_element _array_index) _needweighting
    (switch Utilities|FlowControl|Switch|SwitchonE_Tasks _array_element
      (:NewEnumerator0
        (Variables|DecreaseRates|SetHungerDecreaseRate (Math|Conversions|ToFloat(Integer) (- (Utilities|Array|Length _needweighting) _array_index))))
      (:NewEnumerator1
        (Variables|DecreaseRates|SetSleepDecreaseRate (Math|Conversions|ToFloat(Integer) (- (Utilities|Array|Length _needweighting) _array_index))))
      (:NewEnumerator4
        (Variables|DecreaseRates|SetFellowDecreaseRate (Math|Conversions|ToFloat(Integer) (- (Utilities|Array|Length _needweighting) _array_index))))
      (:NewEnumerator5
        (Variables|DecreaseRates|SetWillDecreaseRate (Math|Conversions|ToFloat(Integer) (- (Utilities|Array|Length _needweighting) _array_index))))))
  (return))

(fn SetStartingSkills
  (for (_array_element _array_index) (Variables|Config|Stats|GetSkillWeighting)
    (switch Utilities|FlowControl|Switch|SwitchonE_Tasks _array_element
      (:NewEnumerator6
        (Variables|Needs|Combat|SetToughness (Math|Conversions|ToFloat(Integer) (Math|Float|Floor (* (Utilities|Array|Get(acopy) (Variables|Default|GetAlphas) _array_index) 1e+01)))))
      (:NewEnumerator7
        (Variables|Needs|Combat|SetWeaponSkill (Math|Conversions|ToFloat(Integer) (Math|Float|Floor (* (Utilities|Array|Get(acopy) (Variables|Default|GetAlphas) _array_index) 1e+01)))))
      (:NewEnumerator8
        (Variables|Needs|Combat|SetEquipment (Math|Conversions|ToFloat(Integer) (Math|Float|Floor (* (Utilities|Array|Get(acopy) (Variables|Default|GetAlphas) _array_index) 1e+01)))))
      (:NewEnumerator9
        (Variables|Needs|Combat|SetSpellCraft (Math|Conversions|ToFloat(Integer) (Math|Float|Floor (* (Utilities|Array|Get(acopy) (Variables|Default|GetAlphas) _array_index) 1e+01)))))))
  (return))

(fn EmptyNeedCheck
  (params (Need :type E_Tasks%20Enum :default "NewEnumerator3") (IsEmpty? :type Boolean))
  (bind _emptyneeds (Variables|Default|GetEmptyNeeds))
  (LocalVariables|SetEmptyCount 0)
  (Utilities|Map|Add _emptyneeds Need IsEmpty?)
  (bind _keys (Utilities|Map|Keys _emptyneeds))
  (for _array_element _keys
    (if (.Value (Utilities|Map|Find (Variables|Default|GetEmptyNeeds) _array_element))
      (Math|Integer|IncrementInt (LocalVariables|GetEmptyCount))))
  (return (>= (LocalVariables|GetEmptyCount) 3)))

(fn SetCustomerName
  (bind _namelist (Variables|Default|GetNameList))
  (bind _outrownames (DataTable|GetDataTableRowNames _namelist))
  (bind _returnvalue (Utilities|GetDataTableRow _namelist (.OutItem (Utilities|Array|Random _outrownames)))
    (:then
      (bind _returnvalue_2 (Utilities|GetDataTableRow _namelist (.OutItem (Utilities|Array|Random _outrownames)) :!label _label)
        (:then
          (if (not (Utilities|Array|IsEmpty (.NameSuffixes (Utilities|Struct|BreakS_CustomerNames _returnvalue_2))))
            (Variables|Default|SetCustomerName (Utilities|Text|FormatText "{First} {Last}" (.NamePrefixes (Utilities|Struct|BreakS_CustomerNames _returnvalue)) (.NameSuffixes (Utilities|Struct|BreakS_CustomerNames _returnvalue_2))))
            (return)
            (else
              (goto _label))))))))

(fn GetWindow
  (Utilities|IsValid (Variables|Default|GetInspectorWindow)
    (:Is%20Valid
      (Default|SetNPCTarget (Variables|Default|GetInspectorWindow) self)
      (return (Variables|Default|GetInspectorWindow) (Variables|/Game/MastersProject/TavernUI/WBP_TavernUI_WindowBase.WBP_TavernUI_WindowBase_C|GetWindowPanel (Variables|/Game/MastersProject/Core/Characters/Customer/WBP_NPCStats.WBP_NPCStats_C|GetWBP_TavernUI_WindowBase (Variables|Default|GetInspectorWindow)))))
    (:Is%20Not%20Valid
      (bind _returnvalue (UserInterface|CreateWidget "/Game/MastersProject/Core/Characters/Customer/WBP_NPCStats.WBP_NPCStats_C"))
      (bind _output_get (Variables|Default|SetInspectorWindow _returnvalue))
      (Default|InitialiseWindow _output_get _output_get)
      (Default|SetNPCTarget _output_get self)
      (return _output_get (Variables|/Game/MastersProject/TavernUI/WBP_TavernUI_WindowBase.WBP_TavernUI_WindowBase_C|GetWindowPanel (Variables|/Game/MastersProject/Core/Characters/Customer/WBP_NPCStats.WBP_NPCStats_C|GetWBP_TavernUI_WindowBase _output_get))))))

(fn IGetQueueIndex
  (return 0))
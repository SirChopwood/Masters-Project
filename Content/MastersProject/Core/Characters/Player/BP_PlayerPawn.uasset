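; BP_PlayerPawn is the player's camera pawn, moved and zoomed through Enhanced Input actions.
; On possession it adds the camera mapping context and caches a reference to the GM_Tavern game mode.
; Forward and right actions feed the floating pawn movement along world axes, while zoom adjusts the spring arm length within clamped limits.
; Two debug keys add or spend currency through the game mode's component and refresh the currency UI.
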(event Input|EnhancedActionEvents|EnhancedInputActionIA_Forward
  (params (ActionValue :type Float%20%28double-precision%29) (ElapsedSeconds :type Float%20%28double-precision%29) (TriggeredSeconds :type Float%20%28double-precision%29) (InputAction :type Input%20Action%20Object%20Reference :default "/Game/MastersProject/Core/Characters/Player/IA_Forward.IA_Forward"))
  ;[1 1 1] Move Forward
  (:Triggered
    (Class|PawnMovementComponent|AddInputVector (Variables|Default|GetFloatingPawnMovement) (Math|Vector|MakeVector ActionValue 0.0 0.0) false)))

(event Input|EnhancedActionEvents|EnhancedInputActionIA_Right
  (params (ActionValue :type Float%20%28double-precision%29) (ElapsedSeconds :type Float%20%28double-precision%29) (TriggeredSeconds :type Float%20%28double-precision%29) (InputAction :type Input%20Action%20Object%20Reference :default "/Game/MastersProject/Core/Characters/Player/IA_Right.IA_Right"))
  ;[1 1 1] Move Right
  (:Triggered
    (Class|PawnMovementComponent|AddInputVector (Variables|Default|GetFloatingPawnMovement) (Math|Vector|MakeVector 0.0 ActionValue 0.0) false)))

(event Input|EnhancedActionEvents|EnhancedInputActionIA_Zoom
  (params (ActionValue :type Float%20%28double-precision%29) (ElapsedSeconds :type Float%20%28double-precision%29) (TriggeredSeconds :type Float%20%28double-precision%29) (InputAction :type Input%20Action%20Object%20Reference :default "/Game/MastersProject/Core/Characters/Player/IA_Zoom.IA_Zoom"))
  ;[1 1 1] Zoom
  (:Triggered
    (Variables|/Script/Engine.SpringArmComponent|SetTargetArmLength (Variables|Default|GetSpringArm) (Math|Float|Clamp(Float) (+ (* ActionValue (Variables|Default|GetZoom%20Strength)) (Variables|/Script/Engine.SpringArmComponent|GetTargetArmLength (Variables|Default|GetSpringArm))) 1e+03 6e+03))))

(event EventPossessed
  (params (NewController :type Controller%20Object%20Reference))
  ;[1 1 1] Add Mapping Context
  (Input|AddMappingContext (PlayerController|LocalPlayerSubsystems|GetEnhancedInputLocalPlayerSubsystem (Game|GetPlayerController 0)) "/Game/MastersProject/Core/Characters/Player/IMC_CameraMovement.IMC_CameraMovement" 0 "(bIgnoreAllPressedKeysUntilRelease=True,bForceImmediately=False)")
  ;[1 1 1] Get Game Mode reference
  (bind _asgm_tavern (Utilities|Casting|CastToGM_Tavern (Game|GetGameMode)))
  (Variables|Default|SetAs%20GM%20Tavern _asgm_tavern))

(event Input|KeyboardEvents|DebugKey2
  (params (Key :type Key%20Structure :default "None") (ActionValue :type Input%20Action%20Value%20Structure))
  (bind _as_gm_tavern (Variables|Default|GetAs%20GM%20Tavern))
  ;[1 1 1] Currency Debug
  (:Pressed
    (bind _success (Default|SpendCurrency (Variables|/Game/MastersProject/Core/GM_Tavern.GM_Tavern_C|GetAC_Currency _as_gm_tavern) 5 "NewEnumerator0"))
    (if _success
      (Default|UpdateUI (Variables|/Game/MastersProject/Core/GM_Tavern.GM_Tavern_C|GetCurrencyUI _as_gm_tavern)))))

(event Input|KeyboardEvents|DebugKey1
  (params (Key :type Key%20Structure :default "None") (ActionValue :type Input%20Action%20Value%20Structure))
  (bind _as_gm_tavern (Variables|Default|GetAs%20GM%20Tavern))
  ;[1 1 1] Currency Debug
  (:Pressed
    (Default|AddCurrency (Variables|/Game/MastersProject/Core/GM_Tavern.GM_Tavern_C|GetAC_Currency _as_gm_tavern) 10 "NewEnumerator0")
    (Default|UpdateUI (Variables|/Game/MastersProject/Core/GM_Tavern.GM_Tavern_C|GetCurrencyUI _as_gm_tavern))))

(fn ConstructionScript)
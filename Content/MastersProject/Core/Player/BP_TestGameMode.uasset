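; BP_TestGameMode is a game mode that tracks a Currency value used to pay for furniture.
; AddCurrency and RemoveCurrency events adjust the balance directly, with no bounds checks.
; CheckIfCurrencyEnough reports whether the balance covers a furniture component's CurrencyCost, without deducting it.
; Two debug keys add or remove fixed amounts for testing.
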(event Custom|Add%20Currency
  (params (AddedCurrency :type Integer))
  (Variables|Default|SetCurrency (+ (Variables|Default|GetCurrency) AddedCurrency)))

(event Custom|Remove%20Currency
  (params (Remove%20Currency :type Integer))
  (Variables|Default|SetCurrency (- (Variables|Default|GetCurrency) Remove%20Currency)))

(event Input|KeyboardEvents|DebugKey1
  (params (Key :type Key%20Structure :default "None") (ActionValue :type Input%20Action%20Value%20Structure))
  (:Pressed
    (CallFunction|AddCurrency 10)))

(event Input|KeyboardEvents|DebugKey2
  (params (Key :type Key%20Structure :default "None") (ActionValue :type Input%20Action%20Value%20Structure))
  (:Pressed
    (CallFunction|RemoveCurrency 5)))

(fn ConstructionScript)

(fn CheckifCurrencyEnough
  (params (FurnitureComponent :type BP%20Furniture%20Component%202%20Object%20Reference))
  (if (<= (Variables|/Game/MastersProject/Core/FurnitureSystem/BP_FurnitureComponent2.BP_FurnitureComponent2_C|GetCurrencyCost FurnitureComponent) (Variables|Default|GetCurrency))
    (return true)
    (else
      (return false))))
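; BP_PlayerPawn is the player's camera pawn, providing planar panning and zoom.
; On BeginPlay it adds the IMC_CameraMovement Enhanced Input mapping context to the first player controller.
; Forward and right actions feed FloatingPawnMovement along fixed world X and Y axes, independent of view rotation.
; The zoom action adjusts the spring arm length by a scaled input, clamped to a fixed range.
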(event Input|EnhancedActionEvents|EnhancedInputActionIA_Forward
  (params (ActionValue :type Float%20%28double-precision%29) (ElapsedSeconds :type Float%20%28double-precision%29) (TriggeredSeconds :type Float%20%28double-precision%29) (InputAction :type Input%20Action%20Object%20Reference :default "/Game/MastersProject/Core/Player/IA_Forward.IA_Forward"))
  ;[1 1 1] Move Forward
  (:Triggered
    (Class|PawnMovementComponent|AddInputVector (Variables|Default|GetFloatingPawnMovement) (Math|Vector|MakeVector ActionValue 0.0 0.0) false)))

(event Input|EnhancedActionEvents|EnhancedInputActionIA_Right
  (params (ActionValue :type Float%20%28double-precision%29) (ElapsedSeconds :type Float%20%28double-precision%29) (TriggeredSeconds :type Float%20%28double-precision%29) (InputAction :type Input%20Action%20Object%20Reference :default "/Game/MastersProject/Core/Player/IA_Right.IA_Right"))
  ;[1 1 1] Move Right
  (:Triggered
    (Class|PawnMovementComponent|AddInputVector (Variables|Default|GetFloatingPawnMovement) (Math|Vector|MakeVector 0.0 ActionValue 0.0) false)))

(event Input|EnhancedActionEvents|EnhancedInputActionIA_Zoom
  (params (ActionValue :type Float%20%28double-precision%29) (ElapsedSeconds :type Float%20%28double-precision%29) (TriggeredSeconds :type Float%20%28double-precision%29) (InputAction :type Input%20Action%20Object%20Reference :default "/Game/MastersProject/Core/Player/IA_Zoom.IA_Zoom"))
  ;[1 1 1] Zoom
  (:Triggered
    (Variables|/Script/Engine.SpringArmComponent|SetTargetArmLength (Variables|Default|GetSpringArm) (Math|Float|Clamp(Float) (+ (* ActionValue (Variables|Default|GetZoom%20Strength)) (Variables|/Script/Engine.SpringArmComponent|GetTargetArmLength (Variables|Default|GetSpringArm))) 1e+03 6e+03))))

(event EventBeginPlay
  ;[1 1 1] Add Mapping Context
  (Input|AddMappingContext (PlayerController|LocalPlayerSubsystems|GetEnhancedInputLocalPlayerSubsystem (Game|GetPlayerController 0)) "/Game/MastersProject/Core/Player/IMC_CameraMovement.IMC_CameraMovement" 0 "(bIgnoreAllPressedKeysUntilRelease=True,bForceImmediately=False)"))

(fn ConstructionScript)